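; Team- and territory-specific soldier spawner for InkGuard that creates spearman or Daka soldiers above its cylinder during the main game.
; Once that mode starts, it registers with SpawnMgr, decides whether it is an enemy spawner, and spawns its MTSpawnInfos list as local or enemy classes.
; Each tick, enemy spawners feed received SpawnMgr data to their soldiers through interface messages, while friendly spawners record soldier HP for sending.
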(event `self.ReceiveBeginPlay`
  (`parent.ReceiveBeginPlay`)
  (`self.Begin Play Initailize`))

(event `self.ReceiveTick`
  (params (DeltaSeconds :type "Float (single-precision)"))
  (bind _spawnmgr (`self.SpawnMgr`))
  (set `self.TimeDelta` DeltaSeconds)
  (if (`self.bInitialized`)
    (bind _returnvalue (`InkGuardGameMode.GetCurGameMode` (`self.As Ink Guard Game Mode`)))
    (switch `EMainGameState` _returnvalue
      (:`GAME_MAINGAME`
        (if (`self.bEnemySpawner`)
          (for (_array_element _array_index) (`self.m_tSpawnInfos`)
            (bind (_ispawntype _ispawnmgrindex) (break `SpawnDutyStruct` _array_element))
            ;[1 1 1] Recv Loop
            (if (`SpawnMgr.IsOtherDataUpdate` _spawnmgr _ispawnmgrindex)
              (bind _returnvalue_2 (`SpawnMgr.GetOtherData` _spawnmgr _ispawnmgrindex))
              (bind _output (`|GetArrayItem` (`self.m_pCharaters`) _array_index))
              (`/Engine/EditorBlueprintResources/StandardMacros.IsValid` _output
                (:`Is Valid`
                  (message `SoldierInterface.SetValueOfPacket` _output _returnvalue_2)))
              (else
                (message `SoldierInterface.SpawnerTick` _output (`self.TimeDelta`)))))
          (else
            (for (_array_element_2 _array_index_2) (`self.m_tSpawnInfos`)
              ;[1 1 1] Send Loop
              (bind _returnvalue_3 (message `SoldierInterface.GetHP` (`|GetArrayItem` (`self.m_pCharaters`) _array_index_2)))
              (bind (_ispawntype_2 _ispawnmgrindex_2) (break `SpawnDutyStruct` _array_element_2))
              (`|VariableSetRef` _array_element_2 (make `SpawnDutyStruct` _ispawntype_2 _ispawnmgrindex_2 _returnvalue_3)))))))
    (else
      (`KismetSystemLibrary.Delay` 1.0)
      (bind _returnvalue_4 (`InkGuardGameMode.GetCurGameMode` (`self.As Ink Guard Game Mode`)))
      (switch `EMainGameState` _returnvalue_4
        (:`GAME_MAINGAME`
          (`self.Stand By Spawn`)
          (`self.Spawn All Object`)
          (set `self.bInitialized` true))))))

(event `self.AppendNewDuty`
  (params (iSoldierType :type Integer) (iSpawnMgrIndex :type Integer))
  ;[1 1 1] AppendDuty
  (bind _output_get (set `self.Temp` (make `SpawnDutyStruct` iSoldierType iSpawnMgrIndex)))
  (`KismetArrayLibrary.Array_Add` (`self.m_tSpawnInfos`) _output_get))

(fn `Begin Play Initailize`
  (bind _asink_guard_game_mode (cast `InkGuardGameMode` (`GameplayStatics.GetGameMode`)))
  (set `self.As Ink Guard Game Mode` _asink_guard_game_mode)
  (set `self.Spwner Name` (`KismetStringLibrary.Concat_StrStr` (`|GetEnumeratorNameAsString` (`self.eTargetTerritoryType`)) "      " (`|GetEnumeratorNameAsString` (`self.eSpawnerColor`)))))

(fn `GetHP`
  (returns (ReturnValue :type "Float (single-precision)"))
  (return 0.0))

(fn `GetRespawn Point`
  (returns (ReturnValue :type "Transform Structure"))
  (bind (_returnvalue_location _returnvalue_rotation) (`KismetMathLibrary.BreakTransform` (`SceneComponent.K2_GetComponentToWorld` (`self.NoCapCylinder`))))
  (return (`KismetMathLibrary.MakeTransform` (+ _returnvalue_location (0.0 0.0 110.0)) _returnvalue_rotation)))

(fn `GetSoldierTypeForCpp`
  (returns (ReturnValue :type Integer))
  (return 0))

(fn `Initailize Construct`
  (locals (NewTargetTerritoryValue :type Integer) (NewTeamColorValue :type Integer))
  ;[1 0.02652 0] Set To Parent
  (switch `/Game/InkGuard/Enums/BP_TerritoryType` (`self.eTargetTerritoryType`)
    (:`NewEnumerator0`
      (set `local.NewTargetTerritoryValue` 0))
    (:`NewEnumerator1`
      (set `local.NewTargetTerritoryValue` 1))
    (:`NewEnumerator4`
      (set `local.NewTargetTerritoryValue` 2))
    (:`NewEnumerator5`
      (set `local.NewTargetTerritoryValue` 3)))
  (switch `/Game/InkGuard/Enums/BP_GameTeam` (`self.eSpawnerColor`)
    (:`NewEnumerator3`
      (set `local.NewTeamColorValue` 0))
    (:`NewEnumerator0`
      (set `local.NewTeamColorValue` 1))
    (:`NewEnumerator1`
      (set `local.NewTeamColorValue` 2)))
  (set `self.iTargetTerritoryType` (`local.NewTargetTerritoryValue`))
  (set `self.iSpawnerColor` (`local.NewTeamColorValue`)))

(fn `IsDead`
  (returns (ReturnValue :type Boolean))
  (return false))

(fn `IsOurTeam`
  (returns (ReturnValue :type Boolean))
  (return false))

(fn `Print Debug Struct`
  (for _array_element (`self.m_tSpawnInfos`)
    (`KismetSystemLibrary.PrintString` (`KismetStringLibrary.Concat_StrStr` (`self.Spwner Name`) "         " (`KismetStringLibrary.Conv_IntToString` (`.iSpawnType` (break `SpawnDutyStruct` _array_element)))) true true (struct :`R` 1.0 :`G` 0.675771 :`A` 1.0))))

(fn `SetColor`
  (bind _nocapcylinder (`self.NoCapCylinder`))
  (switch `/Game/InkGuard/Enums/BP_GameTeam` (`self.eSpawnerColor`)
    (:`NewEnumerator1`
      (bind _returnvalue (`PrimitiveComponent.CreateDynamicMaterialInstance` _nocapcylinder 0 "/Game/InkGuard/MapBP/Object/SpawnPoint/Mesh/MI_NoCapCylinder.MI_NoCapCylinder" "None"))
      (`MaterialInstanceDynamic.SetVectorParameterValue` _returnvalue "TeamColor" (struct :`G` 3.893328 :`B` 50.0 :`A` 1.0))
      (`PrimitiveComponent.SetMaterial` _nocapcylinder 0 _returnvalue))))

(fn `Spawn All Object`
  (locals (SpawnCharacterClass :type "Character Class Reference") (`For loop Struct` :type "SpawnDutyStruct Structure") (LoopIndex :type Integer))
  (bind (_for_loop_struct_ispawntype _for_loop_struct_ispawnmgrindex) (break `SpawnDutyStruct` (`local.For loop Struct`)))
  (bind _benemyspawner (`self.bEnemySpawner`))
  (for (_array_element _array_index) (`self.m_tSpawnInfos`)
    (set `local.LoopIndex` _array_index)
    ;[1 1 1] 지금은 0번 spearman, 1번 daka
    (set `local.For loop Struct` _array_element)
    (switch `int` (`.iSpawnType` (break `SpawnDutyStruct` _array_element))
      (:`0`
        (if _benemyspawner
          (set `local.SpawnCharacterClass` "/Game/InkGuard/EnemyBP/SpearMan/BP_EnemySpearMan.BP_EnemySpearMan_C")
          (else
            (set `local.SpawnCharacterClass` "/Game/InkGuard/EnemyBP/SpearMan/BP_SpearMan.BP_SpearMan_C"))))
      (:`1`
        (if _benemyspawner
          (set `local.SpawnCharacterClass` "/Game/InkGuard/Daka/BP_EnemyDaka.BP_EnemyDaka_C")
          (else
            (set `local.SpawnCharacterClass` "/Game/InkGuard/Daka/BP_Daka.BP_Daka_C")))))
    (bind _returnvalue (`self.GetRespawn Point`))
    (bind _returnvalue_2 (`|SpawnActorFromClass` (`local.SpawnCharacterClass`) (`KismetMathLibrary.MakeTransform` (.location _returnvalue) (.rotation _returnvalue)) "AdjustIfPossibleButAlwaysSpawn" "MultiplyWithRoot" null null))
    (if (`KismetSystemLibrary.DoesImplementInterface` _returnvalue_2 "/Script/InkGuard.SoldierInterface")
      (message `SoldierInterface.SetAboutColor` _returnvalue_2 (`self.iSpawnerColor`))
      (message `SoldierInterface.SetAboutSpawner` _returnvalue_2 self)
      (`KismetArrayLibrary.Array_Set` (`self.m_tSpawnInfos`) (`local.LoopIndex`) (make `SpawnDutyStruct` _for_loop_struct_ispawntype _for_loop_struct_ispawnmgrindex))
      (`KismetArrayLibrary.Array_Add` (`self.m_pCharaters`) _returnvalue_2))))

(fn `Stand By Spawn`
  (bind _returnvalue (`GameplayStatics.GetActorOfClass` "/Script/InkGuard.SpawnMgr"))
  (bind _output_get (set `self.SpawnMgr` _returnvalue))
  (`SpawnMgr.RegisterSpawner` _output_get self (`self.iSpawnerColor`) (`self.iTargetTerritoryType`))
  (bind _bredcolor (`InkGuardGameMode.GetTeamColor` (`self.As Ink Guard Game Mode`)))
  (switch `/Game/InkGuard/Enums/BP_GameTeam` (`self.eSpawnerColor`)
    (:`NewEnumerator3`
      (if (not _bredcolor)
        (set `self.bEnemySpawner` true)))
    (:`NewEnumerator1`
      (if _bredcolor
        (set `self.bEnemySpawner` true)))))

(fn `UserConstructionScript`
  (`self.Initailize Construct`)
  (`self.SetColor`))