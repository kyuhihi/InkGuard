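; Gondola that travels along a three-point quadratic Bezier path once Depart is set, flagging Arrive at the end and tracking riders with an inner trigger.
; The construction script samples the same curve to lay a chain, cycling through five instanced mesh components.
; Tick advances the body, hung below the curve, while a looping timer steps its material's "X" parameter.
; A separate function spawns a Niagara disappear effect below the end point.
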(event `self.ReceiveBeginPlay`
  (`parent.ReceiveBeginPlay`)
  (`KismetSystemLibrary.K2_SetTimer` null "Change AllogDallog" (`self.Material Change Time`) true))

(event `self.ReceiveTick`
  (params (DeltaSeconds :type "Float (single-precision)"))
  (if (`self.Depart`)
    (`self.UpdateBazierLocation` DeltaSeconds)
    (`self.CheckEndPoint`)))

(event `self.InnerTrigger.OnComponentBeginOverlap`
  (params (OverlappedComponent :type "PrimitiveComponent Object Reference") (OtherActor :type "Actor Object Reference") (OtherComp :type "PrimitiveComponent Object Reference") (OtherBodyIndex :type Integer) (bFromSweep :type Boolean) (SweepResult :type "HitResult Structure (by ref)"))
  (set `self.bSomeOneRide` true))

(event `self.InnerTrigger.OnComponentEndOverlap`
  (params (OverlappedComponent :type "PrimitiveComponent Object Reference") (OtherActor :type "Actor Object Reference") (OtherComp :type "PrimitiveComponent Object Reference") (OtherBodyIndex :type Integer))
  (set `self.bSomeOneRide` false))

(fn `Change AllogDallog`
  (bind _changescalarparam (`self.ChangeScalarParam`))
  (bind _returnvalue (+ (`self.ChangeScalarParam`) -0.2))
  (if (< _returnvalue 0.0)
    (`|VariableSetRef` _changescalarparam 1.0)
    (else
      (`|VariableSetRef` _changescalarparam _returnvalue)))
  (`MeshComponent.SetScalarParameterValueOnMaterials` (`self.Body`) "X" (`self.ChangeScalarParam`)))

(fn `CheckEndPoint`
  (if (>= (`self.MoveFollowingBazierTime`) 1.0)
    (set `self.MoveFollowingBazierTime` 1.0)
    (set `self.Arrive` true)
    (`self.UpdateBazierLocation` 0.0)))

(fn `SpawnDisappearEffect`
  (locals (EffectPos :type "Vector Structure"))
  (bind (_effectpos_x _effectpos_y _effectpos_z) (`KismetMathLibrary.BreakVector` (`local.EffectPos`)))
  (bind _output_get (set `local.EffectPos` (`|GetArrayItem` (`self.BazierPoint`) 2)))
  (`self.UpdateToWorldVector` _output_get)
  (`NiagaraFunctionLibrary.SpawnSystemAtLocation` "/Game/InkGuard/MapBP/Object/Gondola/Effect/NS_Disappear.NS_Disappear" (`KismetMathLibrary.MakeVector` _effectpos_x _effectpos_y (+ _effectpos_z -500.0)) (struct) (2.0 2.0 2.0) true true "AutoRelease"))

(fn `UpdateBazierLocation`
  (params (fDeltaTime :type "Float (double-precision)"))
  (locals (BazierPos :type "Vector Structure" :default (0.0 0.0 0.0)))
  (bind _bazierpoint (`self.BazierPoint`))
  (bind _newparam (`self.Get Location Bazier` (`|GetArrayItem` _bazierpoint) (`|GetArrayItem` _bazierpoint 1) (`|GetArrayItem` _bazierpoint 2) (`self.MoveFollowingBazierTime`)))
  (bind _output_get (set `local.BazierPos` _newparam))
  (`self.UpdateToWorldVector` _output_get)
  (`SceneComponent.K2_SetWorldLocation` (`self.Body`) (- (`local.BazierPos`) (0.0 0.0 896.0)) false true)
  (set `self.MoveFollowingBazierTime` (+ (`self.MoveFollowingBazierTime`) (* fDeltaTime 0.3))))

(fn `UserConstructionScript`
  (locals (TopPosition :type "Vector Structure" :default (0.0 0.0 0.0)) (BazierPlusValue :type "Float (double-precision)") (InstanceNum :type Integer) (TargetMesh :type "InstancedStaticMeshComponent Object Reference") (BazierPos :type "Vector Structure"))
  (bind _bazierpoint (`self.BazierPoint`))
  (bind _bazierplusvalue (`local.BazierPlusValue`))
  (bind _placedmesh (`self.PlacedMesh`))
  (`|VariableSetRef` (`|GetArrayItem` (`self.BazierPoint`)) (`local.TopPosition`))
  ;[1 0.1173 0] For Chain
  (`StaticMeshComponent.SetStaticMesh` (`self.InstancedStaticMesh`) (`|GetArrayItem` _placedmesh))
  (`StaticMeshComponent.SetStaticMesh` (`self.InstancedStaticMesh1`) (`|GetArrayItem` _placedmesh 1))
  (`StaticMeshComponent.SetStaticMesh` (`self.InstancedStaticMesh2`) (`|GetArrayItem` _placedmesh 2))
  (`StaticMeshComponent.SetStaticMesh` (`self.InstancedStaticMesh3`) (`|GetArrayItem` _placedmesh 3))
  (`StaticMeshComponent.SetStaticMesh` (`self.InstancedStaticMesh4`) (`|GetArrayItem` _placedmesh 4))
  (while (<= _bazierplusvalue 0.99)
    (bind _newparam (`self.Get Location Bazier` (`|GetArrayItem` _bazierpoint) (`|GetArrayItem` _bazierpoint 1) (`|GetArrayItem` _bazierpoint 2) _bazierplusvalue))
    (bind _output_get (set `local.BazierPos` _newparam))
    (`self.UpdateToWorldVector` _output_get)
    (bind _result (`/Engine/EditorBlueprintResources/StandardMacros.IncrementInt` (`local.InstanceNum`))
      (:`  `
        (bind _returnvalue (mod _result 5))
        (switch `int` _returnvalue
          (:`0`
            (set `local.TargetMesh` (`self.InstancedStaticMesh`)))
          (:`1`
            (set `local.TargetMesh` (`self.InstancedStaticMesh1`)))
          (:`2`
            (set `local.TargetMesh` (`self.InstancedStaticMesh2`)))
          (:`3`
            (set `local.TargetMesh` (`self.InstancedStaticMesh3`)))
          (:`4`
            (set `local.TargetMesh` (`self.InstancedStaticMesh4`))))
        (`InstancedStaticMeshComponent.AddInstance` (`local.TargetMesh`) (`KismetMathLibrary.MakeTransform` (`local.BazierPos`) (struct) (0.2 0.2 0.2)) true)
        (`MeshComponent.SetScalarParameterValueOnMaterials` (`local.TargetMesh`) "X" (* _returnvalue 0.2))
        (set `local.BazierPlusValue` (+ (`local.BazierPlusValue`) 0.016))))))