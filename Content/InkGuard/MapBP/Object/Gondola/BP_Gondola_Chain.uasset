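; BP_Gondola_Chain is a gondola chain actor that animates the material color of five instanced static mesh components.
; A looping timer runs ChangeColor, which steps each stored scalar down by 0.2, wrapping to 1 below zero, then writes each to its component's "X" material parameter.
; It also defines quadratic Bezier and local-to-world helpers, though its graphs never call them and the construction script is empty.
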(event `self.ReceiveBeginPlay`
  (`KismetSystemLibrary.K2_SetTimer` null "ChangeColor" (`self.Material Change Time`) true))

(fn `ChangeColor`
  (bind _material_scalar_parms (`self.Material Scalar Parms`))
  (`self.Increse Scalar`
    (:`Completed`
      (`MeshComponent.SetScalarParameterValueOnMaterials` (`self.InstancedStaticMesh`) "X" (`|GetArrayItem` _material_scalar_parms))
      (`MeshComponent.SetScalarParameterValueOnMaterials` (`self.InstancedStaticMesh1`) "X" (`|GetArrayItem` _material_scalar_parms 1))
      (`MeshComponent.SetScalarParameterValueOnMaterials` (`self.InstancedStaticMesh2`) "X" (`|GetArrayItem` _material_scalar_parms 2))
      (`MeshComponent.SetScalarParameterValueOnMaterials` (`self.InstancedStaticMesh3`) "X" (`|GetArrayItem` _material_scalar_parms 3))
      (`MeshComponent.SetScalarParameterValueOnMaterials` (`self.InstancedStaticMesh4`) "X" (`|GetArrayItem` _material_scalar_parms 4)))))

(fn `Get Location Bazier`
  (params (Start :type "Vector Structure") (Anchor :type "Vector Structure") (End :type "Vector Structure") (Time :type "Float (double-precision)"))
  (returns (NewParam :type "Vector Structure"))
  (locals (TempA :type "Vector Structure" :default (0.0 0.0 0.0)) (TempB :type "Vector Structure" :default (0.0 0.0 0.0)))
  (`|ExecutionSequence`
    (:`then_0`
      (set `local.TempB` (`KismetMathLibrary.VLerp` Anchor End Time))
      (set `local.TempA` (`KismetMathLibrary.VLerp` Start Anchor Time)))
    (:`then_1`
      (return (`KismetMathLibrary.VLerp` (`local.TempA`) (`local.TempB`) Time)))))

(fn `UpdateToWorldVector`
  (params (`In Vector` :type "Vector Structure (by ref)"))
  (`|VariableSetRef` `In Vector` (`KismetMathLibrary.TransformLocation` (`self.GetTransform`) `In Vector`)))

(fn `UserConstructionScript`
  (locals (BazierPlusValue :type "Float (double-precision)") (InstanceNum :type Integer) (BazierPos :type "Vector Structure" :default (0.0 0.0 0.0)) (TargetMesh :type "InstancedStaticMeshComponent Object Reference")))