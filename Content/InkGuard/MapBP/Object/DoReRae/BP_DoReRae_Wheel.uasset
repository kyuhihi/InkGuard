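; Interactive wheel for the DoReRae map object that an overlapping character spins by holding F to build up a fill gauge.
; While the key is held, Tick eases wheel speed up, raises the widget material's fill progress, records the character's team color and triggers their animation.
; Releasing slows the wheel and drains the gauge; an externally set SpillTiming flag overrides input and drains it five times faster.
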(event `self.ReceiveTick`
  (params (DeltaSeconds :type "Float (single-precision)"))
  (bind _overlapcharacter (`self.OverlapCharacter`))
  (`/Engine/EditorBlueprintResources/StandardMacros.IsValid` _overlapcharacter
    (:`Is Valid`
      (if (`self.bSpillTiming`)
        (`self.FillWaterUI` true (* DeltaSeconds 5.0))
        (`self.CalculateWheelSpeed` false DeltaSeconds)
        (else
          (bind _returnvalue (message `PlayerInterface.AboutKeyPressingF` _overlapcharacter))
          (`self.FillWaterUI` (not _returnvalue) DeltaSeconds)
          (`self.CalculateWheelSpeed` _returnvalue DeltaSeconds)))
      (`self.ExcuteWheelAnimation` DeltaSeconds))
    (:`Is Not Valid`
      (`self.FillWaterUI` true DeltaSeconds))))

(event `self.Box.OnComponentBeginOverlap`
  (params (OverlappedComponent :type "PrimitiveComponent Object Reference") (OtherActor :type "Actor Object Reference") (OtherComp :type "PrimitiveComponent Object Reference") (OtherBodyIndex :type Integer) (bFromSweep :type Boolean) (SweepResult :type "HitResult Structure (by ref)"))
  (if (`KismetSystemLibrary.DoesImplementInterface` OtherActor "/Game/InkGuard/Baku/Mantle.Mantle_C")
    (bind `_as캐릭터` (cast `Character` OtherActor))
    (set `self.OverlapCharacter` `_as캐릭터`)))

(event `self.Box.OnComponentEndOverlap`
  (params (OverlappedComponent :type "PrimitiveComponent Object Reference") (OtherActor :type "Actor Object Reference") (OtherComp :type "PrimitiveComponent Object Reference") (OtherBodyIndex :type Integer))
  (if (== OtherActor (`self.OverlapCharacter`))
    (set `self.OverlapCharacter` null)))

(fn `CalculateWheelSpeed`
  (params (bPressF :type Boolean) (DeltaTime :type "Float (double-precision)"))
  (locals (TargetSpeed :type "Float (double-precision)") (LerpAlpha :type "Float (double-precision)" :default 1.0))
  (if bPressF
    (set `local.TargetSpeed` 400.0)
    (else
      (set `local.TargetSpeed` 0.0)))
  (set `self.WheelSpeed` (`KismetMathLibrary.Lerp` (`self.WheelSpeed`) (`local.TargetSpeed`) (* DeltaTime (`local.LerpAlpha`))))
  (return))

(fn `ExcuteWheelAnimation`
  (params (A :type "Float (double-precision)"))
  (`SceneComponent.K2_AddWorldRotation` (`self.Wheel`) (`KismetMathLibrary.MakeRotator` 0.0 (* A (`self.WheelSpeed`))) false false))

(fn `FillWaterUI`
  (params (bMinus :type Boolean) (DeltaTime :type "Float (double-precision)"))
  (`/Engine/EditorBlueprintResources/StandardMacros.IsValid` (`self.WBP_Interaction_Fill`)
    (:`Is Valid`
      _)
    (:`Is Not Valid`
      ;[1 1 1] Get & Set All About UI Instance
      (bind _aswbp_interaction_fill (cast `/Game/InkGuard/UI/2D/WBP_InteractionFill` (`WidgetComponent.GetWidget` (`self.Widget`))))
      (bind _output_get (set `self.WBP_Interaction_Fill` _aswbp_interaction_fill))
      (set `self.WBP_DynamicMaterial` (`WidgetBlueprintLibrary.GetDynamicMaterial` (`Image.Brush` (`/Game/InkGuard/UI/2D/WBP_InteractionFill.Image_76` _output_get))))))
  (if bMinus
    (set `self.InteractionTime` (`KismetMathLibrary.FMax` (- (`self.InteractionTime`) DeltaTime)))
    (else
      ;[1 1 1] 증가하는 중이라면 칼라를 Set해준다.
      (bind _returnvalue (message `PlayerInterface.GetColor` (`self.OverlapCharacter`)))
      (bind _newparam (`self.Int to EGameTeam` _returnvalue))
      (set `self.TargetColor` _newparam)
      (message `PlayerInterface.DoreraeAnimation` (`self.OverlapCharacter`))
      (set `self.InteractionTime` (`KismetMathLibrary.FMin` (+ DeltaTime (`self.InteractionTime`)) (`self.MaxBlendTime`)))))
  (bind _output_get_2 (set `self.ProgressPercent` (`KismetMathLibrary.FMin` (/ (`self.InteractionTime`) (`self.MaxBlendTime`)) 1.0)))
  (`MaterialInstanceDynamic.SetScalarParameterValue` (`self.WBP_DynamicMaterial`) "Fill progress" _output_get_2))

(fn `GetSpillTiming`
  (returns (bSpillTiming :type Boolean))
  (return (`self.bSpillTiming`)))

(fn `Int to EGameTeam`
  (params (TargetColorInt :type Integer))
  (returns (NewParam :type "/Game/InkGuard/Enums/BP_GameTeam Enum"))
  (switch `int` TargetColorInt
    (:`0`
      (return "NewEnumerator3"))
    (:`1`
      (return "NewEnumerator0"))
    (:`2`
      (return "NewEnumerator1"))))

(fn `SetSpillTiming`
  (params (bSpill :type Boolean))
  (set `self.bSpillTiming` bSpill))

(fn `UserConstructionScript`)