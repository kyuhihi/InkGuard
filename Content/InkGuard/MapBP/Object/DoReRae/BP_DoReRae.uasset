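; BP_DoReRae is a pulley-style water bottle prop that fills from a spawned wheel's progress and spills when full.
; On BeginPlay it spawns the BP_DoReRae_Wheel and creates a dynamic material for the bottle's inner water.
; Tick maps wheel progress to water alpha and height, sets the wheel's spill flag at max height, and eases the spill angle.
; The angle reveals the waterfall mesh, then triggers a guarded, timed reset.
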(event `self.ReceiveBeginPlay`
  ;[1 1 1] SetUp Mesh and Dynamic Material
  (bind _returnvalue (`self.GenerateWoodAndWheel` (`self.MakeWheelLocation` -190.0)))
  (set `self.WheelR` _returnvalue)
  (bind _returnvalue_2 (`PrimitiveComponent.CreateDynamicMaterialInstance` (`self.Bottle`) 0 "/Game/InkGuard/MapBP/Object/DoReRae/MI_WaterInner.MI_WaterInner" "None"))
  (set `self.BottleInnerMat` _returnvalue_2))

(event `self.ReceiveTick`
  (params (DeltaSeconds :type "Float (single-precision)"))
  (`/Engine/EditorBlueprintResources/StandardMacros.IsValid` (`self.WheelR`)
    (:`Is Valid`
      (`self.SetWaterAlpha` DeltaSeconds)
      (`self.SetSurfaceOfWater`)
      (`self.MakeSpillAngle` DeltaSeconds)
      (bind _spillfinishtiming (`self.CheckSpillTiming`))
      (if _spillfinishtiming
        (`self.Tidy Spill Finish Routine`)))))

(event `Tidy Spill Finish Routine`
  (if (not (`self.bTidyRoutine`))
    (`KismetSystemLibrary.K2_SetTimerDelegate` (delegate `Set_Initialize`) 3.0)
    (set `self.bTidyRoutine` true)))

(event `Set_Initialize`
  (`/Game/InkGuard/MapBP/Object/DoReRae/BP_DoReRae_Wheel.SetSpillTiming` (`self.WheelR`) false)
  (`self.Render Water Fall` false)
  (`KismetSystemLibrary.Delay` 3.0)
  (set `self.bTidyRoutine` false))

(fn `CheckSpillTiming`
  (returns (SpillFinishTiming :type Boolean))
  (locals (MaxHeight :type "Float (double-precision)" :default 199.5) (MaxSpillAngle :type "Float (double-precision)" :default 119.0))
  (bind _bspilltiming (`/Game/InkGuard/MapBP/Object/DoReRae/BP_DoReRae_Wheel.GetSpillTiming` (`self.WheelR`)))
  (if _bspilltiming
    (return (>= (`self.SpillAngle`) (`local.MaxSpillAngle`)))
    (else
      (`/Game/InkGuard/MapBP/Object/DoReRae/BP_DoReRae_Wheel.SetSpillTiming` (`self.WheelR`) (>= (`self.WaterHeight`) (`local.MaxHeight`))))))

(fn `GenerateWoodAndWheel`
  (params (RelativeLocation :type "Vector Structure") (bLeftWheel :type Boolean))
  (returns (ReturnValue :type "/Game/InkGuard/MapBP/Object/DoReRae/BP_DoReRae_Wheel Object Reference"))
  (locals (RelativeRotation :type "Rotator Structure" :default (struct)))
  (bind _returnvalue (`|SpawnActorFromClass` "/Game/InkGuard/MapBP/Object/DoReRae/BP_DoReRae_Wheel.BP_DoReRae_Wheel_C" (`KismetMathLibrary.MakeRelativeTransform` (`KismetMathLibrary.Conv_VectorToTransform` (`self.K2_GetActorLocation`)) (`KismetMathLibrary.MakeTransform` RelativeLocation (`KismetMathLibrary.MakeRotator` 0.0))) "AlwaysSpawn" "MultiplyWithRoot" null null))
  (if bLeftWheel
    (bind _returnvalue_2 (`self.MakeWheelRotation` -1.0 _returnvalue)
      (:`excute2`
        (`self.K2_SetActorRotation` _returnvalue _returnvalue_2 false)))
    (else
      (bind _returnvalue_3 (`self.MakeWheelRotation` 1.0 _returnvalue)
        (:`excute2`
          (`self.K2_SetActorRotation` _returnvalue _returnvalue_3 false)))))
  (return _returnvalue))

(fn `MakeSpillAngle`
  (params (DeltaTime :type "Float (double-precision)"))
  (locals (TargetAngle :type "Float (double-precision)"))
  (bind _returnvalue (`KismetMathLibrary.FInterpEaseInOut` (`self.SpillAngle`) (`local.TargetAngle`) DeltaTime 0.8))
  (bind _bspilltiming (`/Game/InkGuard/MapBP/Object/DoReRae/BP_DoReRae_Wheel.GetSpillTiming` (`self.WheelR`)))
  (if _bspilltiming
    (set `local.TargetAngle` 120.0)
    (bind _output_get (set `self.SpillAngle` _returnvalue))
    (if (>= _output_get 106.0)
      (`self.Render Water Fall` true))
    (else
      (set `local.TargetAngle` 0.0)
      (set `self.SpillAngle` _returnvalue))))

(fn `Render Water Fall`
  (params (bRender :type Boolean))
  (`SceneComponent.SetVisibility` (`self.FallMiddle`) bRender true))

(fn `SetSurfaceOfWater`
  (locals (fMultipleVar :type "Float (double-precision)" :default 190.0) (fPlusVar :type "Float (double-precision)" :default 10.0))
  (bind _wheelr (`self.WheelR`))
  (bind _bspilltiming (`/Game/InkGuard/MapBP/Object/DoReRae/BP_DoReRae_Wheel.GetSpillTiming` _wheelr))
  (if _bspilltiming
    (set `local.fMultipleVar` 310.0)
    (set `local.fPlusVar` -110.0)
    (else
      (set `local.fMultipleVar` 190.0)
      (set `local.fPlusVar` 10.0)))
  (set `self.WaterHeight` (+ (* (`/Game/InkGuard/MapBP/Object/DoReRae/BP_DoReRae_Wheel.ProgressPercent` _wheelr) (`local.fMultipleVar`)) (`local.fPlusVar`)))
  (`MaterialInstanceDynamic.SetScalarParameterValue` (`self.BottleInnerMat`) "Scale" (`self.WaterHeight`)))

(fn `SetWaterAlpha`
  (params (Alpha :type "Float (double-precision)"))
  (locals (TargetWaterAlpha :type "Float (double-precision)") (MultipleVar :type "Float (double-precision)" :default 5.0))
  (bind _wheelr (`self.WheelR`))
  (bind _returnvalue (`KismetMathLibrary.Lerp` (`self.WaterAlpha`) (`local.TargetWaterAlpha`) (* Alpha (`local.MultipleVar`))))
  (bind _bspilltiming (`/Game/InkGuard/MapBP/Object/DoReRae/BP_DoReRae_Wheel.GetSpillTiming` _wheelr))
  (if _bspilltiming
    (set `local.MultipleVar` 0.5)
    (else
      (set `local.MultipleVar` 5.0)))
  (if (<= (`/Game/InkGuard/MapBP/Object/DoReRae/BP_DoReRae_Wheel.ProgressPercent` _wheelr) 0.0)
    (set `local.TargetWaterAlpha` 0.0)
    (set `self.WaterAlpha` _returnvalue)
    (else
      (set `local.TargetWaterAlpha` 1.0)
      (set `self.WaterAlpha` _returnvalue)))
  (`MaterialInstanceDynamic.SetScalarParameterValue` (`self.BottleInnerMat`) "WaterAlpha" (`self.WaterAlpha`)))

(fn `UserConstructionScript`)