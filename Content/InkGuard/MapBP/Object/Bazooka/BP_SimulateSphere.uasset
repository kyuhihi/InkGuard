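; BP_SimulateSphere is a physics ball used by a bazooka's simulation, exploding visually on contact.
; SetSimulatingPawnAndOwner stores the bazooka owner and simulating pawn, clears the collision flag, and makes the ball visible and physics-driven.
; Overlaps on CollisionSphere ignore both references and itself; any other spawns an explosion emitter, sets the flag, hides and freezes the ball, then calls TidySimulating on the owner.
; The ball is never destroyed here, so setup can re-arm it.
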(event `self.CollisionSphere.OnComponentBeginOverlap`
  (params (OverlappedComponent :type "PrimitiveComponent Object Reference") (OtherActor :type "Actor Object Reference") (OtherComp :type "PrimitiveComponent Object Reference") (OtherBodyIndex :type Integer) (bFromSweep :type Boolean) (SweepResult :type "HitResult Structure (by ref)"))
  (if (and (and (!= OtherActor (`self.SimulatingPawn`)) (!= OtherActor (`self.BazookaOwner`))) (!= OtherActor self))
    (`GameplayStatics.SpawnEmitterAtLocation` "/Game/StarterContent/Particles/P_Explosion.P_Explosion" (`SceneComponent.K2_GetComponentLocation` (`self.Ball`)))
    (set `self.bCollisionSomeWhere` true)
    (`SceneComponent.SetVisibility` (`self.Ball`) false false)
    (`PrimitiveComponent.SetSimulatePhysics` (`self.Ball`) false)
    (`/Game/InkGuard/MapBP/Object/Bazooka/BP_Bazooka.TidySimulating` (`self.BazookaOwner`))))

(fn `SetSimulatingPawnAndOwner`
  (params (BazookaOwner :type "/Game/InkGuard/MapBP/Object/Bazooka/BP_Bazooka Object Reference") (SimulatingPawn :type "Pawn Object Reference"))
  (set `self.BazookaOwner` BazookaOwner)
  (set `self.SimulatingPawn` SimulatingPawn)
  (set `self.bCollisionSomeWhere` false)
  (`PrimitiveComponent.SetSimulatePhysics` (`self.Ball`) true)
  (`SceneComponent.SetVisibility` (`self.Ball`) true false))

(fn `UserConstructionScript`)