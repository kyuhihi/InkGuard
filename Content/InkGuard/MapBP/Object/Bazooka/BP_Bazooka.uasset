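; Possessable bazooka cannon that a player enters by holding F nearby, then aims to launch their own pawn.
; Tick drives the billboard hold-progress widget and camera blend, and rebuilds a predicted arc from spline components with a landing marker.
; Timers on WASD adjust pitch and yaw; left click flags shooting.
; The Shoot event repossesses the pawn, which then follows a launched BP_SimulateSphere physics ball each tick while simulating.
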(event `self.ReceiveTick`
  (params (DeltaSeconds :type "Float (single-precision)"))
  (bind _pathpoints (`self.PathPoints`))
  (set `self.DeltaTime` DeltaSeconds)
  (`ActorComponent.K2_DestroyComponent` _pathpoints)
  (`KismetArrayLibrary.Array_Clear` _pathpoints)
  (`SplineComponent.ClearSplinePoints` (`self.PredictLine`) true)
  (`self.ManageSpringArm`)
  (`self.DrawProjectile`)
  (`self.UIBillBoard`)
  (`self.CheckFKeyPress` (`self.DeltaTime`))
  (`self.FillProgressUI`)
  (if (`self.bSimulating`)
    (`self.K2_SetActorLocation` (`self.PawnRef`) (`SceneComponent.K2_GetComponentLocation` (`/Game/InkGuard/MapBP/Object/Bazooka/BP_SimulateSphere.Ball` (`self.SimulateBall`))) false true)
    (else
      (set `self.CanShoot` true)
      (`self.AboutPossess`))))

(event `Key|F`
  (params (Key :type "Key Structure"))
  ;[1 1 1] UnPossess
  (:`Pressed`
    (`self.UnPossess` false)))

(event `Key|LeftMouseButton`
  (params (Key :type "Key Structure"))
  ;[1 1 1] Shoot
  (:`Pressed`
    (if (`self.CanShoot`)
      (set `self.CanShoot` false)
      (set `self.IsShooting` true)
      (`KismetSystemLibrary.Delay` 0.2)
      (set `self.IsShooting` false))))

(event `self.InteractionTrigger.OnComponentBeginOverlap`
  (params (OverlappedComponent :type "PrimitiveComponent Object Reference") (OtherActor :type "Actor Object Reference") (OtherComp :type "PrimitiveComponent Object Reference") (OtherBodyIndex :type Integer) (bFromSweep :type Boolean) (SweepResult :type "HitResult Structure (by ref)"))
  ;[1 1 1] About Trigger
  (bind `_as폰` (cast `Pawn` OtherActor))
  (if (`self.IsPlayerControlled` `_as폰`)
    (cast `/Game/InkGuard/MapBP/Object/Bazooka/BP_Bazooka` `_as폰`
      (:`CastFailed`
        (set `self.PawnRef` `_as폰`)
        (set `self.Can be Possessed` true)))))

(event `self.InteractionTrigger.OnComponentEndOverlap`
  (params (OverlappedComponent :type "PrimitiveComponent Object Reference") (OtherActor :type "Actor Object Reference") (OtherComp :type "PrimitiveComponent Object Reference") (OtherBodyIndex :type Integer))
  ;[1 1 1] About Trigger
  (if (== OtherActor (`self.PawnRef`))
    (if (not (`self.bSimulating`))
      (set `self.PawnRef` null)
      (set `self.Can be Possessed` false))))

(event `Key|W`
  (params (Key :type "Key Structure"))
  ;[1 1 1] AimUp
  (:`Pressed`
    (if (`KismetSystemLibrary.K2_IsTimerActiveHandle` (`self.AimUpTimerHandle`))
      (`KismetSystemLibrary.K2_ClearAndInvalidateTimerHandle` (`self.AimUpTimerHandle`) :!label _label)
      (else
        (bind _returnvalue (`KismetSystemLibrary.K2_SetTimerDelegate` (delegate `AimUp`) 0.01 true))
        (set `self.AimUpTimerHandle` _returnvalue))))
  (:`Released`
    (goto _label)))

(event `AimUp`
  ;[1 1 1] AimUp
  (bind _output_get (set `self.Pitch` (`KismetMathLibrary.FClamp` (+ (`self.Pitch`) (* (`self.DeltaTime`) (`self.PitchSpeed`))) 0.0 70.0)))
  (`KismetSystemLibrary.PrintString` (`KismetStringLibrary.Conv_DoubleToString` _output_get)))

(event `Shoot`
  ;[1 1 1] Shoot
  (`self.UnPossess` true))

(event `Key|S`
  (params (Key :type "Key Structure"))
  ;[1 1 1] AimDown
  (:`Pressed`
    (if (`KismetSystemLibrary.K2_IsTimerActiveHandle` (`self.AimDownTimerHandle`))
      (`KismetSystemLibrary.K2_ClearAndInvalidateTimerHandle` (`self.AimDownTimerHandle`) :!label _label_2)
      (else
        (bind _returnvalue (`KismetSystemLibrary.K2_SetTimerDelegate` (delegate `AimDown`) 0.01 true))
        (set `self.AimDownTimerHandle` _returnvalue))))
  (:`Released`
    (goto _label_2)))

(event `Key|One`
  (params (Key :type "Key Structure"))
  ;[1 1 1] Camera toggles
  (:`Pressed`
    (`ActorComponent.Activate` (`self.CameraSide`) false)
    (`ActorComponent.Deactivate` (`self.Camera`))))

(event `AimDown`
  ;[1 1 1] AimDown
  (bind _output_get (set `self.Pitch` (`KismetMathLibrary.FClamp` (- (`self.Pitch`) (* (`self.PitchSpeed`) (`self.DeltaTime`))) 0.0 70.0)))
  (`KismetSystemLibrary.PrintString` (`KismetStringLibrary.Conv_DoubleToString` _output_get)))

(event `Key|Two`
  (params (Key :type "Key Structure"))
  ;[1 1 1] Camera toggles
  (:`Pressed`
    (`ActorComponent.Activate` (`self.Camera`) false)
    (`ActorComponent.Deactivate` (`self.CameraSide`))))

(event `Key|A`
  (params (Key :type "Key Structure"))
  ;[1 1 1] AimLeft
  (:`Pressed`
    (if (`KismetSystemLibrary.K2_IsTimerActiveHandle` (`self.AimLeftTimerHandle`))
      (`KismetSystemLibrary.K2_ClearAndInvalidateTimerHandle` (`self.AimLeftTimerHandle`) :!label _label_3)
      (else
        (bind _returnvalue (`KismetSystemLibrary.K2_SetTimerDelegate` (delegate `AimLeft`) 0.01 true))
        (set `self.AimLeftTimerHandle` _returnvalue))))
  (:`Released`
    (goto _label_3)))

(event `AimLeft`
  ;[1 1 1] AimLeft
  (`SceneComponent.K2_AddWorldRotation` (`self.Bazooka`) (`KismetMathLibrary.MakeRotator` 0.0 0.0 -1.0) false false))

(event `Key|D`
  (params (Key :type "Key Structure"))
  ;[1 1 1] AimRight
  (:`Pressed`
    (if (`KismetSystemLibrary.K2_IsTimerActiveHandle` (`self.AimRightTimerHandle`))
      (`KismetSystemLibrary.K2_ClearAndInvalidateTimerHandle` (`self.AimRightTimerHandle`) :!label _label_4)
      (else
        (bind _returnvalue (`KismetSystemLibrary.K2_SetTimerDelegate` (delegate `AimRight`) 0.01 true))
        (set `self.AimRightTimerHandle` _returnvalue))))
  (:`Released`
    (goto _label_4)))

(event `AimRight`
  ;[1 1 1] AimRight
  (`SceneComponent.K2_AddWorldRotation` (`self.Bazooka`) (`KismetMathLibrary.MakeRotator` 0.0 0.0 1.0) false false))

(fn `CheckFKeyPress`
  (params (fTimeDelta :type "Float (double-precision)"))
  (bind _returnvalue (`GameplayStatics.GetPlayerController` 0))
  (if (`self.Can be Possessed`)
    (if (not (`self.bPossess`))
      (if (`PlayerController.WasInputKeyJustPressed` _returnvalue "F")
        (set `self.bPressedF` true))
      (if (`PlayerController.WasInputKeyJustReleased` _returnvalue "F")
        (set `self.bPressedF` false))
      (if (`self.bPressedF`)
        (set `self.InteractionTimer` (+ fTimeDelta (`self.InteractionTimer`)))
        (else
          (set `self.InteractionTimer` 0.0))))))

(fn `DrawProjectile`
  (bind _bazooka (`self.Bazooka`))
  (bind _shootpositionsock (`self.ShootPositionSock`))
  (bind _gridsphere (`self.GridSphere`))
  (bind _predictline (`self.PredictLine`))
  (bind _gridsphere_2 (`self.GridSphere`))
  (if (`self.bPossess`)
    (`SceneComponent.SetVisibility` _gridsphere_2 true false)
    (bind (_outhit _outpathpositions _outlasttracedestination) (`GameplayStatics.Blueprint_PredictProjectilePath_ByObjectType` :`StartPos` (`SceneComponent.GetSocketLocation` _bazooka _shootpositionsock) :`LaunchVelocity` (* (`SceneComponent.GetSocketRotation` _bazooka _shootpositionsock) (`self.ShootSpeed`)) :`ProjectileRadius` 20.0 :`ObjectTypes` (`|MakeArray` "ObjectTypeQuery1" :!type "EObjectTypeQuery Enum") :`SimFrequency` 10.0 :`MaxSimTime` 10.0))
    (for (_array_element _array_index) _outpathpositions
      (bind _returnvalue (`KismetArrayLibrary.Array_LastIndex` _outpathpositions))
      (if (not (== _array_index (- _returnvalue 1)))
        (`SplineComponent.AddSplinePointAtIndex` _predictline _array_element _array_index "World" true)))
    (`SplineComponent.SetSplinePointType` _predictline _returnvalue "CurveClamped" true)
    (for (_ _array_index_2) _outpathpositions
      (bind _returnvalue_2 (`AddComponent|NODE_AddSplineMeshComponent-1` :`bManualAttachment` true))
      (`KismetArrayLibrary.Array_Add` (`self.PathPoints`) _returnvalue_2)
      (`SceneComponent.SetMobility` _returnvalue_2 "Movable")
      (`SceneComponent.K2_SetWorldLocation` _returnvalue_2 (`SplineComponent.GetLocationAndTangentAtSplinePoint` (`self.PredictLine`) _array_index_2 "World") false true)
      (`SceneComponent.SetWorldScale3D` _returnvalue_2 (0.3 0.1 0.1))
      (`SceneComponent.K2_SetWorldLocation` _gridsphere (`KismetMathLibrary.VInterpTo` (`SceneComponent.K2_GetComponentLocation` _gridsphere) _outlasttracedestination (`GameplayStatics.GetWorldDeltaSeconds`) 10.0) false false))
    (else
      (`SceneComponent.SetVisibility` _gridsphere_2 false false))))

(fn `FillProgressUI`
  (locals (ProgressValue :type "Float (double-precision)"))
  (bind _aswbp_interaction_fill (cast `/Game/InkGuard/UI/2D/WBP_InteractionFill` (`WidgetComponent.GetWidget` (`self.FillUI`))))
  (if (`self.bPossess`)
    (set `local.ProgressValue` 1.0)
    (else
      (bind _output_get (set `local.ProgressValue` (/ (`self.InteractionTimer`) (`self.MaxBlendTime`))))))
  (`MaterialInstanceDynamic.SetScalarParameterValue` (`WidgetBlueprintLibrary.GetDynamicMaterial` (`Image.Brush` (`/Game/InkGuard/UI/2D/WBP_InteractionFill.Image_76` _aswbp_interaction_fill))) "Fill progress" _output_get))

(fn `ManageSpringArm`
  (locals (MinSpringArm :type "Float (double-precision)") (MaxSpringArm :type "Float (double-precision)" :default 1142.0) (TargetSpringArmLength :type "Float (double-precision)"))
  (bind _springarm (`self.SpringArm`))
  (if (`self.bPossess`)
    (set `local.TargetSpringArmLength` (`local.MinSpringArm`))
    (set `local.TargetSpringArmLength` (`KismetMathLibrary.Lerp` (`SpringArmComponent.TargetArmLength` _springarm) (`local.TargetSpringArmLength`) (* (`self.DeltaTime`) 5.0)))
    (else
      (set `local.TargetSpringArmLength` (`local.MaxSpringArm`))))
  (set `SpringArmComponent.TargetArmLength` (`local.TargetSpringArmLength`) _springarm))

(fn `TidySimulating`
  (set `self.CanShoot` false)
  (set `self.bPossess` false)
  (set `self.bSimulating` false)
  (`self.ManageSpringArm`))

(fn `UIBillBoard`
  (bind _fillui (`self.FillUI`))
  (`SceneComponent.SetVisibility` _fillui (`self.Can be Possessed`) false)
  (`SceneComponent.K2_SetWorldRotation` _fillui (`KismetMathLibrary.FindLookAtRotation` (`SceneComponent.K2_GetComponentLocation` (`self.FillUI`)) (`PlayerCameraManager.GetCameraLocation` (`GameplayStatics.GetPlayerCameraManager` 0))) false false))

(fn `UserConstructionScript`)