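; Bazooka effect actor that shows Chaos debris from a geometry collection, then dissolves and removes it.
; On BeginPlay it applies a strong upward impulse to the geometry collection and waits a few seconds.
; A fast looping timer then steps down the material's Dissolve scalar parameter and destroys the actor once the value drops below zero.
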(event `self.ReceiveBeginPlay`
  (`PrimitiveComponent.AddImpulse` (`self.GeometryCollectionComponent`) (0.0 0.0 100000.0) "None" false)
  (`KismetSystemLibrary.Delay` 3.0)
  (`KismetSystemLibrary.K2_SetTimerDelegate` (delegate `Disssolve`) 0.01 true))

(event `Disssolve`
  (bind _output_get (set `self.DissolveVal` (- (`self.DissolveVal`) 0.016)))
  (`MeshComponent.SetScalarParameterValueOnMaterials` (`self.GeometryCollectionComponent`) "Dissolve" _output_get)
  (if (< _output_get 0.0)
    (`self.K2_DestroyActor`)))

(fn `UserConstructionScript`)