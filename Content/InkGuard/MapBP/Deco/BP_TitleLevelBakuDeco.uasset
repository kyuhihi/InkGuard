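; BP_TitleLevelBakuDeco is a decorative Baku actor for the title level that plays a title animation on demand.
; PlayTitleBakuAnim chains three PlayMontageBaku calls, each starting when the previous one blends out.
; PlayMontageBaku plays AM_TitleBaku at half speed from a section named in MontageNames.
; When the last named section blends out, it sets the mesh play rate to zero to freeze the animation.
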(event `self.ReceiveTick`
  (params (DeltaSeconds :type "Float (single-precision)")))

(event `Play TitleBaku Anim`
  (`self.PlayMontageBaku` 0
    (:`블렌드 아웃 시`
      (`self.PlayMontageBaku` 1
        (:`블렌드 아웃 시`
          (`self.PlayMontageBaku` 2))))))

(fn `UserConstructionScript`)