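; Rectangular capture-area marker labelled "B" that displays the ink progress and color of its territory on a world widget and a fight-place icon.
; It finds the matching BP_DoReRae_Wheel by owner type, then copies its progress and color to both widgets each tick, with extra recoloring during spill timing.
; An overlap box counts pawns to raise or lower the icon, and hides the world widget while BP_Baku is inside.
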(event `self.ReceiveBeginPlay`
  (bind _aswbp_fight_place_ink_icon_square_inner (cast `/Game/InkGuard/UI/2D/WBP_FightPlace_InkIcon_Square_Inner` (`WidgetComponent.GetWidget` (`self.UI`))))
  (bind _output_get (set `self.As WBP Fight Place Ink Icon Square Inner` _aswbp_fight_place_ink_icon_square_inner))
  (`/Game/InkGuard/UI/2D/WBP_FightPlace_InkIcon_Square_Inner.Modify Text` _output_get "B")
  (`self.Set Wheel` "NewEnumerator1"))

(event `self.ReceiveTick`
  (params (DeltaSeconds :type "Float (single-precision)"))
  (bind _fightplace_icon (`self.Fightplace Icon`))
  (if (> (`self.inAreaCnt`) 0)
    (`/Game/InkGuard/UI/2D/WBP_FightPlace_InkIcon_Square.Set Icon Up` _fightplace_icon)
    (else
      (`/Game/InkGuard/UI/2D/WBP_FightPlace_InkIcon_Square.Set Icon Down` _fightplace_icon)))
  (`SceneComponent.SetVisibility` (`self.UI`) (`self.RenderUI`) false)
  (`self.Sync UI Percent And Color`))

(event `self.OverlapSize Cube.OnComponentBeginOverlap`
  (params (OverlappedComponent :type "PrimitiveComponent Object Reference") (OtherActor :type "Actor Object Reference") (OtherComp :type "PrimitiveComponent Object Reference") (OtherBodyIndex :type Integer) (bFromSweep :type Boolean) (SweepResult :type "HitResult Structure (by ref)"))
  (cast `Pawn` OtherActor)
  (`/Engine/EditorBlueprintResources/StandardMacros.IncrementInt` (`self.inAreaCnt`)
    (:`  `
      (cast `/Game/InkGuard/Baku/BP_Baku` OtherActor)
      (set `self.RenderUI` false))))

(event `self.OverlapSize Cube.OnComponentEndOverlap`
  (params (OverlappedComponent :type "PrimitiveComponent Object Reference") (OtherActor :type "Actor Object Reference") (OtherComp :type "PrimitiveComponent Object Reference") (OtherBodyIndex :type Integer))
  (cast `Pawn` OtherActor)
  (`/Engine/EditorBlueprintResources/StandardMacros.DecrementInt` (`self.inAreaCnt`)
    (:`  `
      (cast `/Game/InkGuard/Baku/BP_Baku` OtherActor)
      (set `self.RenderUI` true))))

(event `/Game/InkGuard/MapBP/FillColorInterface.Fill Progress`
  (params (NewPercent :type "Float (double-precision)"))
  (`/Game/InkGuard/UI/2D/WBP_FightPlace_InkIcon_Square_Inner.SetProgressPercent` (`self.As WBP Fight Place Ink Icon Square Inner`) NewPercent))

(event `/Game/InkGuard/MapBP/FillColorInterface.SetColor`
  (params (`New Color` :type "/Game/InkGuard/Enums/BP_GameTeam Enum" :default "NewEnumerator3")))

(fn `Set Wheel`
  (params (`Territory type` :type "/Game/InkGuard/MapBP/Object/DoReRae/E_DoreraeType Enum" :default "NewEnumerator0"))
  (bind _outactors (`GameplayStatics.GetAllActorsOfClass` "/Game/InkGuard/MapBP/Object/DoReRae/BP_DoReRae_Wheel.BP_DoReRae_Wheel_C"))
  (for _array_element _outactors
    (bind _asbp_do_re_rae (cast `/Game/InkGuard/MapBP/Object/DoReRae/BP_DoReRae` (`self.GetOwner` _array_element)))
    (if (`|EnumEquality` `Territory type` (`/Game/InkGuard/MapBP/Object/DoReRae/BP_DoReRae.DoreraeType` _asbp_do_re_rae))
      (set `self.Territory Wheel` _array_element))))

(fn `Sync UI Percent And Color`
  (bind _as_wbp_fight_place_ink_icon_square_inner (`self.As WBP Fight Place Ink Icon Square Inner`))
  (bind _territory_wheel (`self.Territory Wheel`))
  (bind _targetcolor (`/Game/InkGuard/MapBP/Object/DoReRae/BP_DoReRae_Wheel.TargetColor` _territory_wheel))
  (bind _wbp_fightplace_inkicon_square_inner_72 (`/Game/InkGuard/UI/2D/WBP_FightPlace_InkIcon_Square.WBP_FightPlace_InkIcon_Square_Inner_72` (`self.Fightplace Icon`)))
  (bind _progresspercent (`/Game/InkGuard/MapBP/Object/DoReRae/BP_DoReRae_Wheel.ProgressPercent` _territory_wheel))
  (`/Engine/EditorBlueprintResources/StandardMacros.IsValid` (`self.Territory Wheel`)
    (:`Is Valid`
      _)
    (:`Is Not Valid`
      (`self.Set Wheel` "NewEnumerator1")))
  (`/Game/InkGuard/UI/2D/WBP_FightPlace_InkIcon_Square_Inner.SetProgressPercent` _as_wbp_fight_place_ink_icon_square_inner _progresspercent)
  (`/Game/InkGuard/UI/2D/WBP_FightPlace_InkIcon_Square_Inner.SetProgressPercent` _wbp_fightplace_inkicon_square_inner_72 _progresspercent)
  (`/Game/InkGuard/UI/2D/WBP_FightPlace_InkIcon_Square_Inner.SetColor` _as_wbp_fight_place_ink_icon_square_inner _targetcolor true)
  (`/Game/InkGuard/UI/2D/WBP_FightPlace_InkIcon_Square_Inner.SetColor` _wbp_fightplace_inkicon_square_inner_72 _targetcolor true)
  (bind _bspilltiming (`/Game/InkGuard/MapBP/Object/DoReRae/BP_DoReRae_Wheel.GetSpillTiming` (`self.Territory Wheel`)))
  (if _bspilltiming
    (`/Game/InkGuard/UI/2D/WBP_FightPlace_InkIcon_Square_Inner.SetColor` (`self.As WBP Fight Place Ink Icon Square Inner`) _targetcolor false)
    (`/Game/InkGuard/UI/2D/WBP_FightPlace_InkIcon_Square_Inner.SetColor` (`/Game/InkGuard/UI/2D/WBP_FightPlace_InkIcon_Square.WBP_FightPlace_InkIcon_Square_Inner_72` (`self.Fightplace Icon`)) _targetcolor false)))

(fn `UserConstructionScript`)