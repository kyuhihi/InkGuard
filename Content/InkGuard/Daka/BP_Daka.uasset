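; Daka, an AI sword soldier that fights for either team in InkGuard, with health bar, minimap dot and kill-log reporting.
; The behavior tree triggers a four-section montage combo, with timer-looped sphere traces dealing sword damage.
; Hits from the opposing team cause ink effects and knockback; death spawns a death-animation actor and respawns it at its spawner or saved position.
; Enemy copies mirror position, speed, HP and montage time from received packets.
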(event `self.ReceiveBeginPlay`
  ;[1 1 1] Begin!
  ;;[1 1 1] UI
  (bind _aswb_spear_man_health_bar (cast `/Game/InkGuard/Baku/WB_SpearManHealthBar` (`WidgetComponent.GetWidget` (`self.Health Bar Widget`))))
  (set `self.HealthBar UI` _aswb_spear_man_health_bar)
  (set `self.Montage_Attack` "/Game/InkGuard/Daka/Animations/Daka_Attack_ComboMongtage.Daka_Attack_ComboMongtage")
  (`self.Begin Color`)
  (`self.SetTargetDoReRae`)
  (`self.MainGame Routine`
    (:`GAME_MAINGAME`
      (`KismetSystemLibrary.K2_SetTimerDelegate` (delegate `Check Only MainGame Actor`) 3.0))))

(event `Check Only MainGame Actor`
  ;[1 1 1] Begin!
  (`/Engine/EditorBlueprintResources/StandardMacros.IsValid` (`self.My Spawner`)
    (:`Is Not Valid`
      (`self.K2_DestroyActor`))))

(event `self.ReceiveTick`
  (params (DeltaSeconds :type "Float (single-precision)"))
  (`self.SetHpBarBillboard`)
  (if (not (`self.bEnemyDaka`))
    (set `self.Speed` (`KismetMathLibrary.VSize` (`MovementComponent.Velocity` (`self.CharacterMovement`))))))

(event `self.PawnSensing.OnSeePawn`
  (params (Pawn :type "Pawn Object Reference"))
  ;[0.151 0.151 0.151] 보류
)

(event `FollowPlayer`
  ;[0.151 0.151 0.151] 보류
  (if (`self.isSeeingPlayer?`)
    (`/Engine/EditorBlueprintResources/StandardMacros.IsValid` (`self.TestDoreRAE`)
      (:`Is Valid`
        (`AIController.MoveToLocation` (`AIBlueprintHelperLibrary.GetAIController` self) (`self.K2_GetActorLocation` (`self.TestDoreRAE`)) -1.0 true true false true null true)))))

(event `Attack1`
  ;[0.151 0.151 0.151] Combo System
  ;;[0.151 0.151 0.151] Attack1
  (`/Engine/EditorBlueprintResources/StandardMacros.DoOnce` false :!label _label
    (:`Completed`
      (`KismetSystemLibrary.Delay` 0.1)
      (`|PlayMontage` (`self.Mesh`) "/Game/InkGuard/Daka/Animations/Daka_Attack_ComboMongtage.Daka_Attack_ComboMongtage" 1.0 0.0 "Combo1"
        (:`then`
          (set `self.attack Index` 1)
          (goto _label :!via `Reset`))))))

(event `Sword Attack Combo Call From BT`
  (params (targetToAttack :type "Actor Object Reference"))
  (bind (_returnvalue_roll _returnvalue_pitch _returnvalue_yaw) (`KismetMathLibrary.BreakRotator` (`KismetMathLibrary.FindLookAtRotation` (`self.K2_GetActorLocation`) (`self.K2_GetActorLocation` targetToAttack))))
  ;[0.151 0.151 0.151] Combo System
  ;;[0.151 0.151 0.151] Attack Input
  (`self.K2_SetActorRotation` (`KismetMathLibrary.MakeRotator` 0.0 0.0 _returnvalue_yaw))
  (if (`self.can Attack?`)
    (`self.Sword Attack`)))

(event `Attack2`
  ;[0.151 0.151 0.151] Combo System
  ;;[0.151 0.151 0.151] Attack2
  (`/Engine/EditorBlueprintResources/StandardMacros.DoOnce` false :!label _label_2
    (:`Completed`
      (`KismetSystemLibrary.Delay` 0.1)
      (`|PlayMontage` (`self.Mesh`) "/Game/InkGuard/Daka/Animations/Daka_Attack_ComboMongtage.Daka_Attack_ComboMongtage" 1.0 0.0 "Combo2"
        (:`then`
          (set `self.attack Index` 2)
          (goto _label_2 :!via `Reset`))))))

(event `Sword Attack`
  ;[0.151 0.151 0.151] Combo System
  ;;[0.151 0.151 0.151] Sword Attack
  (if (`self.is Attacking?`)
    (set `self.save Attack?` true)
    (else
      (set `self.is Attacking?` true)
      (switch `int` (`self.attack Index`) :!label _label_3
        (:`0`
          (`self.Attack1`))
        (:`1`
          (`self.Attack2`))
        (:`2`
          (`self.Attack3`))
        (:`3`
          (`self.Attack4`))))))

(event `Sword Attack Combo`
  ;[0.151 0.151 0.151] Combo System
  ;;[0.151 0.151 0.151] Combo Continue
  (if (`self.save Attack?`)
    (set `self.save Attack?` false)
    (goto _label_3)
    (else
      (`self.Stop Combo`))))

(event `Attack3`
  ;[0.151 0.151 0.151] Combo System
  ;;[0.151 0.151 0.151] Attack3
  (`/Engine/EditorBlueprintResources/StandardMacros.DoOnce` false :!label _label_4
    (:`Completed`
      (`KismetSystemLibrary.Delay` 0.1)
      (`|PlayMontage` (`self.Mesh`) "/Game/InkGuard/Daka/Animations/Daka_Attack_ComboMongtage.Daka_Attack_ComboMongtage" 1.0 0.0 "Combo3"
        (:`then`
          (set `self.attack Index` 3)
          (goto _label_4 :!via `Reset`))))))

(event `Stop Combo`
  ;[0.151 0.151 0.151] Combo System
  ;;[0.151 0.151 0.151] Stop Combo/ Attack
  (set `self.is Attacking?` false)
  (set `self.attack Index` 0))

(event `Attack4`
  ;[0.151 0.151 0.151] Combo System
  ;;[0.151 0.151 0.151] Attack4
  (`/Engine/EditorBlueprintResources/StandardMacros.DoOnce` false :!label _label_5
    (:`Completed`
      (`KismetSystemLibrary.Delay` 0.1)
      (`|PlayMontage` (`self.Mesh`) "/Game/InkGuard/Daka/Animations/Daka_Attack_ComboMongtage.Daka_Attack_ComboMongtage" 1.0 0.0 "Combo4"
        (:`then`
          (set `self.attack Index` 4)
          (goto _label_5 :!via `Reset`))))))

(event `Start Sword Trace`
  ;[0.151 0.151 0.151] Sword Trace
  (bind _returnvalue (`KismetSystemLibrary.K2_SetTimerDelegate` (delegate `Sword Trace Loop`) 0.001 true))
  (set `self.SwordTraceLoop` _returnvalue))

(event `Sword Trace Loop`
  ;[0.151 0.151 0.151] Sword Trace
  (bind (_outhit _returnvalue) (`KismetSystemLibrary.SphereTraceSingle` (`SceneComponent.K2_GetComponentLocation` (`self.Sword Top Point`)) (`SceneComponent.K2_GetComponentLocation` (`self.Sword Bottom Point`)) 12.0 "TraceTypeQuery4" false (`|MakeArray` (`self.GetOwner`)) "ForDuration" true (struct :`R` 1.0 :`A` 1.0) (struct :`G` 1.0 :`A` 1.0) 0.2))
  (if _returnvalue
    (bind (_bblockinghit _binitialoverlap _time _distance _location _impactpoint _normal _impactnormal _physmat _hitactor) (`GameplayStatics.BreakHitResult` _outhit))
    (if (`self.ActorHasTag` _hitactor "Damageable")
      (`/Engine/EditorBlueprintResources/StandardMacros.DoOnce` false :!label _label_6
        (:`Completed`
          (`GameplayStatics.ApplyDamage` _hitactor 10.0 null self)
          (`KismetSystemLibrary.Delay` 0.1)
          (goto _label_6 :!via `Reset`))))))

(event `Stop Sword Trace`
  ;[0.151 0.151 0.151] Sword Trace
  (`KismetSystemLibrary.K2_ClearAndInvalidateTimerHandle` (`self.SwordTraceLoop`)))

(event `self.ReceiveAnyDamage`
  (params (Damage :type "Float (single-precision)") (DamageType :type "DamageType Object Reference") (InstigatedBy :type "Controller Object Reference") (DamageCauser :type "Actor Object Reference"))
  ;[1 1 1] Damaged
  (if (`KismetSystemLibrary.DoesImplementInterface` DamageCauser "/Script/InkGuard.SoldierInterface")
    (bind _returnvalue (message `SoldierInterface.IsOurTeam` DamageCauser))
    (bind _returnvalue_2 (`self.IsOurTeam`))
    (if (!= _returnvalue_2 _returnvalue)
      (bind (_veffectpoint _returnvalue_3) (message `SoldierInterface.GetEffectPoint` DamageCauser (`self.K2_GetActorLocation` self)))
      (if _returnvalue_3
        (`self.Make Ink Effect` (`KismetMathLibrary.MakeTransform` (.location _veffectpoint) (.rotation _veffectpoint) (.scale _veffectpoint))))
      (`self.SetDamagedLoutine` Damage DamageCauser))))

(event `SoldierInterface.SetAboutSpawner`
  (params (pOwnerSpawner :type "Actor Object Reference"))
  ;[0 1 0.1864] Call By Spawner
  (bind _asbp_soldier_spawner (cast `/Game/InkGuard/MapBP/Object/SpawnPoint/BP_SoldierSpawner` pOwnerSpawner))
  (set `self.My Spawner` _asbp_soldier_spawner))

(event `SoldierInterface.SetAboutColor`
  (params (NewColor :type Integer))
  ;[0 1 0.1864] Call By Spawner
  (switch `int` NewColor
    (:`0`
      (set `self.TeamColor` "NewEnumerator3"))
    (:`1`
      (set `self.TeamColor` "NewEnumerator0"))
    (:`2`
      (set `self.TeamColor` "NewEnumerator1"))))

(event `SoldierInterface.Respawn`
  (bind _braincomponent (`AIController.BrainComponent` (`AIBlueprintHelperLibrary.GetAIController` self)))
  ;[1 0.0111 0] Respawn
  (`/Engine/EditorBlueprintResources/StandardMacros.IsValid` (`self.My Spawner`)
    (:`Is Valid`
      (bind _returnvalue (`/Game/InkGuard/MapBP/Object/SpawnPoint/BP_SoldierSpawner.GetRespawn Point` (`self.My Spawner`)))
      (`self.K2_SetActorTransform` _returnvalue false true))
    (:`Is Not Valid`
      (`self.K2_SetActorTransform` (`self.SaveSpawnerPos`) false true)))
  (`/Game/InkGuard/Baku/BPC/Bpc_PlayerStats.SetHP` (`self.Bpc_PlayerStats`))
  (`/Engine/EditorBlueprintResources/StandardMacros.IsValid` _braincomponent
    (:`Is Valid`
      (`BrainComponent.RestartLogic` _braincomponent))))

(event `SoldierInterface.SetValueOfPacket`
  (params (tRecvPacket :type "PACKET_SOLDIER_TRANSFORM_BLUEPRINT Structure"))
  ;[1 1 1] Packet
  (if (`self.bEnemyDaka`)
    (`self.Sync Movement` tRecvPacket_vSoldier_Position tRecvPacket_fSoldier_Yaw tRecvPacket_fSoldier_Speed)
    (`/Game/InkGuard/Baku/BPC/Bpc_PlayerStats.Sync HP` (`self.Bpc_PlayerStats`) tRecvPacket_fHP)
    ;;[1 0 0.7553] 애니메이션 동기화
    (if (> tRecvPacket_fSoldier_MontagePlayTime 0.0)
      (`|PlayMontage` (`self.Mesh`) (`self.Montage_Attack`) 1.0 tRecvPacket_fSoldier_MontagePlayTime)
      (else
        (`self.Stop Attack Montage`)))))

(event `SoldierInterface.SpawnerTick`
  (params (fTimeDelta :type "Float (single-precision)"))
  (bind (_returnvalue_roll _returnvalue_pitch _returnvalue_yaw) (`KismetMathLibrary.BreakRotator` (`self.GetControlRotation` self)))
  ;[1 1 1] If Without Update
  (if (not (`AnimInstance.IsAnyMontagePlaying` (`SkeletalMeshComponent.GetAnimInstance` (`self.Mesh`))))
    (`self.AddMovementInput` (`KismetMathLibrary.GetForwardVector` (`KismetMathLibrary.MakeRotator` 0.0 0.0 _returnvalue_yaw)))))

(fn `AboutKeyPressingF`
  (returns (ReturnValue :type Boolean))
  (return false))

(fn `Attack`
  (returns (`Animation Duration` :type "Float (double-precision)"))
  (locals (`Target Actor` :type Name :default "Target Actor"))
  (bind _returnvalue (`AIBlueprintHelperLibrary.GetBlackboard` null))
  (`/Engine/EditorBlueprintResources/StandardMacros.IsValid` _returnvalue
    (:`Is Valid`
      (bind `_as액터` (cast `Actor` (`BlackboardComponent.GetValueAsObject` _returnvalue (`local.Target Actor`))))
      (if (`KismetSystemLibrary.DoesImplementInterface` `_as액터` "/Script/InkGuard.SoldierInterface")
        (bind _returnvalue_2 (message `SoldierInterface.IsOurTeam` `_as액터`))
        (bind _returnvalue_3 (`self.IsOurTeam`))
        (if (!= _returnvalue_2 _returnvalue_3)
          (`self.Sword Attack Combo Call From BT` `_as액터`)
          (return 0.4))))))

(fn `Begin Color`
  (locals (Dotui :type "/Game/InkGuard/UI/BP_Minimap_Dot_UI Object Reference"))
  (bind _ink_guard_game_mode (`self.Ink Guard Game Mode`))
  (bind _papersprite (`/Game/InkGuard/UI/BP_Minimap_Dot_UI.PaperSprite` (`local.Dotui`)))
  (bind _asink_guard_game_mode (cast `InkGuardGameMode` (`GameplayStatics.GetGameMode`)))
  (set `self.Ink Guard Game Mode` _asink_guard_game_mode)
  (bind _returnvalue (`|SpawnActorFromClass` "/Game/InkGuard/UI/BP_Minimap_Dot_UI.BP_Minimap_Dot_UI_C" (`self.GetTransform`) "AlwaysSpawn" "MultiplyWithRoot" null null))
  (bind _output_get (set `local.Dotui` _returnvalue))
  (set `/Game/InkGuard/UI/BP_Minimap_Dot_UI.UIOwner` self _output_get)
  (if (`self.bEnemyDaka`)
    (bind _bredcolor (`InkGuardGameMode.GetTeamColor` _ink_guard_game_mode))
    (if (not _bredcolor)
      (`PaperSpriteComponent.SetSprite` _papersprite "/Game/InkGuard/UI/MainMap/Minimap/T_RedCircle_Sprite.T_RedCircle_Sprite" :!label _label)
      (else
        (`PaperSpriteComponent.SetSprite` _papersprite "/Game/InkGuard/UI/MainMap/Minimap/T_BlueCircle_Sprite.T_BlueCircle_Sprite" :!label _label_2)))
    (else
      (bind _bredcolor_2 (`InkGuardGameMode.GetTeamColor` _ink_guard_game_mode))
      (if _bredcolor_2
        (goto _label)
        (else
          (goto _label_2))))))

(fn `GetColor`
  (returns (ReturnValue :type Integer))
  (return 0))

(fn `GetEffectPoint`
  (params (MyLocation :type "Vector Structure"))
  (returns (vEffectPoint :type "Transform Structure") (ReturnValue :type Boolean))
  (bind (_outhit _returnvalue) (`KismetSystemLibrary.LineTraceSingle` :`Start` (`SceneComponent.K2_GetComponentLocation` (`self.Sword`)) :`End` MyLocation :`TraceChannel` "TraceTypeQuery4" :`DrawTime` 15.0))
  (bind (_bblockinghit _binitialoverlap _time _distance _location _impactpoint _normal) (`GameplayStatics.BreakHitResult` _outhit))
  (return (`KismetMathLibrary.MakeTransform` _location (`KismetMathLibrary.MakeRotFromXY` _normal _normal) (1.5 1.5 1.5)) _returnvalue))

(fn `GetHP`
  (returns (ReturnValue :type "Float (single-precision)"))
  (return (`/Game/InkGuard/Baku/BPC/Bpc_PlayerStats.Current Health` (`self.Bpc_PlayerStats`))))

(fn `GetPlayerInputData`
  (returns (ReturnValue :type "PlayerInputStruct Structure"))
  (return))

(fn `GetSoldierTypeForCpp`
  (returns (ReturnValue :type Integer))
  (return (`KismetMathLibrary.Conv_ByteToInt` (enumliteral `/Game/InkGuard/Enums/BP_CharacterEnum` "NewEnumerator4"))))

(fn `IsDead`
  (returns (ReturnValue :type Boolean))
  (return (<= (`/Game/InkGuard/Baku/BPC/Bpc_PlayerStats.Current Health` (`self.Bpc_PlayerStats`)) 0.0)))

(fn `IsOurTeam`
  (returns (ReturnValue :type Boolean))
  (return (not (`self.bEnemyDaka`))))

(fn `Make Ink Effect`
  (params (EffectTransfom :type "Transform Structure"))
  (`GameplayStatics.SpawnEmitterAtLocation` "/Game/Realistic_Starter_VFX_Pack_Vol2/Particles/Blood/P_Blood_Splat_Cone.P_Blood_Splat_Cone" EffectTransfom_Location EffectTransfom_Rotation EffectTransfom_Scale true "AutoRelease"))

(fn `Make System Log`
  (params (DamageCauser :type "Actor Object Reference"))
  (locals (CauserColor :type "/Game/InkGuard/Enums/BP_GameTeam Enum" :default "NewEnumerator3") (CauserCharacter :type "/Game/InkGuard/Enums/BP_CharacterEnum Enum" :default "NewEnumerator3"))
  (`/Engine/EditorBlueprintResources/StandardMacros.IsValid` (`self.Ink Guard Game Mode`)
    (:`Is Valid`
      _)
    (:`Is Not Valid`
      (bind _asink_guard_game_mode (cast `InkGuardGameMode` (`GameplayStatics.GetGameMode`)))
      (set `self.Ink Guard Game Mode` _asink_guard_game_mode)))
  (bind _returnvalue (`InkGuardGameMode.GetCurGameMode` (`self.Ink Guard Game Mode`)))
  (switch `EMainGameState` _returnvalue
    (:`GAME_WAITING`
      ;[1 0 0.00204] CauserColor
      (set `local.CauserColor` "NewEnumerator1"))
    (:`GAME_MAINGAME`
      (bind _bredcolor (`InkGuardGameMode.GetTeamColor` (`self.Ink Guard Game Mode`)))
      (if _bredcolor
        (set `local.CauserColor` "NewEnumerator1")
        (else
          (set `local.CauserColor` "NewEnumerator3")))))
  ;[1 1 1] Enemy Class라면 색변경
  (if (`self.bEnemyDaka`)
    (switch `/Game/InkGuard/Enums/BP_GameTeam` (`local.CauserColor`)
      (:`NewEnumerator3`
        (set `local.CauserColor` "NewEnumerator1"))
      (:`NewEnumerator1`
        (set `local.CauserColor` "NewEnumerator3"))))
  ;[1 0.9194 0] Causer Character
  (bind _returnvalue_2 (message `SoldierInterface.GetSoldierTypeForCpp` DamageCauser))
  (switch `int` _returnvalue_2
    (:`0`
      (set `local.CauserCharacter` "NewEnumerator3"))
    (:`1`
      (set `local.CauserCharacter` "NewEnumerator0"))
    (:`2`
      (set `local.CauserCharacter` "NewEnumerator1"))
    (:`3`
      (set `local.CauserCharacter` "NewEnumerator2"))
    (:`4`
      (set `local.CauserCharacter` "NewEnumerator4")))
  (message `/Game/InkGuard/UI/UI_Interface.Add KillLog` (`self.Ink Guard Game Mode`) (make `/Game/InkGuard/Baku/UI/Notification/Notification_KillLog` (`local.CauserColor`) (`local.CauserCharacter`) "NewEnumerator4")))

(fn `SetDamagedLoutine`
  (params (DamageAmount :type "Float (single-precision)") (DamageCauser :type "Actor Object Reference"))
  (bind _braincomponent (`AIController.BrainComponent` (`AIBlueprintHelperLibrary.GetAIController` self)))
  (`self.LaunchCharacter` (* (`KismetMathLibrary.GetForwardVector` (`self.K2_GetActorRotation` DamageCauser)) 700.0))
  (`self.K2_SetActorRotation` (`KismetMathLibrary.FindLookAtRotation` (`self.K2_GetActorLocation`) (`self.K2_GetActorLocation` DamageCauser)))
  (bind _isplayerdead_ (`/Game/InkGuard/Baku/BPC/Bpc_PlayerStats.Decrease Health` (`self.Bpc_PlayerStats`) DamageAmount))
  (if _isplayerdead_
    ;[1 0 0.04792] Set Dead
    (`self.Make System Log` DamageCauser)
    (`PrimitiveComponent.SetCollisionObjectType` (`self.Mesh`) "ECC_PhysicsBody")
    (`PrimitiveComponent.SetSimulatePhysics` (`self.Mesh`) true)
    (`|SpawnActorFromClass` "/Game/InkGuard/Daka/BP_AIDakadeadAnimation.BP_AIDakadeadAnimation_C" (`self.GetTransform`) "AdjustIfPossibleButAlwaysSpawn" "MultiplyWithRoot" null null)
    (`/Engine/EditorBlueprintResources/StandardMacros.IsValid` _braincomponent
      (:`Is Valid`
        (`BrainComponent.StopLogic` _braincomponent ""))
      (:`Is Not Valid`
        _))
    (`self.Respawn`)))

(fn `SetTargetDoReRae`
  (bind _returnvalue (`AIBlueprintHelperLibrary.GetBlackboard` null))
  (`/Engine/EditorBlueprintResources/StandardMacros.IsValid` (`AIBlueprintHelperLibrary.GetBlackboard` null)
    (:`Is Valid`
      (bind _outactors (`GameplayStatics.GetAllActorsOfClass` "/Game/InkGuard/MapBP/Object/DoReRae/BP_DoReRae.BP_DoReRae_C"))
      (for _array_element _outactors
        (switch `/Game/InkGuard/MapBP/Object/DoReRae/E_DoreraeType` (`/Game/InkGuard/MapBP/Object/DoReRae/BP_DoReRae.DoreraeType` _array_element)
          (:`NewEnumerator0`
            (`BlackboardComponent.SetValueAsObject` _returnvalue "DoReRaeA" _array_element))
          (:`NewEnumerator1`
            (`BlackboardComponent.SetValueAsObject` _returnvalue "DoReRaeB" _array_element))
          (:`NewEnumerator2`
            (`BlackboardComponent.SetValueAsObject` _returnvalue "DoReRaeC" _array_element)))))))

(fn `Stop Attack Montage`
  (bind _returnvalue (`AnimInstance.GetCurrentActiveMontage` (`SkeletalMeshComponent.GetAnimInstance` (`self.Mesh`))))
  (`self.Stop Combo`)
  (`/Engine/EditorBlueprintResources/StandardMacros.IsValid` _returnvalue
    (:`Is Valid`
      (`self.StopAnimMontage` _returnvalue))))

(fn `Sync Movement`
  (params (NewLocation :type "Vector Structure") (NewRotation_Yaw :type "Float (single-precision)") (NewSpeed :type "Float (double-precision)"))
  (bind (_returnvalue_roll _returnvalue_pitch) (`KismetMathLibrary.BreakRotator` (`self.K2_GetActorRotation`)))
  (`self.K2_SetActorLocation` NewLocation false true)
  (`self.K2_SetActorRotation` (`KismetMathLibrary.MakeRotator` _returnvalue_roll _returnvalue_pitch NewRotation_Yaw) true)
  (set `self.Speed` NewSpeed))

(fn `UserConstructionScript`)