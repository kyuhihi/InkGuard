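; BP_BallistaArrow is the arrow actor for the ballista, handling what happens when it strikes something.
; When its Collision component begins an overlap with anything other than itself or its instigator, it turns on physics simulation for the static mesh.
; Each such overlap also spawns a bullet impact particle effect at the collision component's location, with a counter capping the spawns at three per arrow.
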(event `self.Collision.OnComponentBeginOverlap`
  (params (OverlappedComponent :type "PrimitiveComponent Object Reference") (OtherActor :type "Actor Object Reference") (OtherComp :type "PrimitiveComponent Object Reference") (OtherBodyIndex :type Integer) (bFromSweep :type Boolean) (SweepResult :type "HitResult Structure (by ref)"))
  (if (and (!= OtherActor (`self.GetInstigator`)) (!= OtherActor self))
    (`PrimitiveComponent.SetSimulatePhysics` (`self.StaticMesh`) true)
    (if (< (`self.SystemsSpawned`) 3)
      (`GameplayStatics.SpawnEmitterAtLocation` "/Game/ART/Effects/ParticleSystems/Gameplay/Player/P_body_bullet_impact.P_body_bullet_impact" (`SceneComponent.K2_GetComponentLocation` OverlappedComponent))
      (`/Engine/EditorBlueprintResources/StandardMacros.IncrementInt` (`self.SystemsSpawned`)))))

(fn `UserConstructionScript`)