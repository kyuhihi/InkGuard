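; Player-possessable ballista pawn that aims and fires arrows.
; Box overlap shows a key prompt and stores the player pawn; Tick polls F to possess the ballista, and F again repossesses that pawn.
; WASD runs looping timers that step clamped pitch and yaw.
; Left click plays shot effects and sets IsShooting; separate Shoot and EndShoot events, not called here, spawn the arrow and re-arm the weapon.
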(event `Key|W`
  (params (Key :type "Key Structure"))
  ;[1 1 1] Vertical rotation (aiming)
  (:`Pressed`
    (if (`KismetSystemLibrary.K2_IsTimerActiveHandle` (`self.AimUpTimerHandle`))
      (`KismetSystemLibrary.K2_ClearAndInvalidateTimerHandle` (`self.AimUpTimerHandle`) :!label _label)
      (else
        (bind _returnvalue (`KismetSystemLibrary.K2_SetTimerDelegate` (delegate `AimUp`) (`self.VerticalAimTime`) true))
        (set `self.AimUpTimerHandle` _returnvalue))))
  (:`Released`
    (goto _label)))

(event `Key|A`
  (params (Key :type "Key Structure"))
  ;[1 1 1] Horizontal Rotation
  (:`Pressed`
    (if (`KismetSystemLibrary.K2_IsTimerActiveHandle` (`self.Aim Left Timer Handle`))
      (`KismetSystemLibrary.K2_ClearAndInvalidateTimerHandle` (`self.Aim Left Timer Handle`) :!label _label_2)
      (else
        (bind _returnvalue (`KismetSystemLibrary.K2_SetTimerDelegate` (delegate `AimLeft`) (`self.HorizontalAimTime`) true))
        (set `self.Aim Left Timer Handle` _returnvalue))))
  (:`Released`
    (goto _label_2)))

(event `AimUp`
  ;[1 1 1] Vertical rotation (aiming)
  (set `self.Pitch` (`KismetMathLibrary.FClamp` (+ (`self.Pitch`) (`self.DeltaAim`)) -60.0 60.0)))

(event `AimLeft`
  ;[1 1 1] Horizontal Rotation
  (set `self.Yaw` (`KismetMathLibrary.FClamp` (- (`self.Yaw`) (`self.DeltaAim`)) -30.0 30.0)))

(event `self.ReceiveTick`
  (params (DeltaSeconds :type "Float (single-precision)"))
  (bind _returnvalue (`GameplayStatics.GetPlayerController` 0))
  ;[1 1 1] Tick (possess)
  (if (and (not (`self.IsPlayerControlled`)) (`self.CanBePossessed`))
    (`/Engine/EditorBlueprintResources/StandardMacros.IsValid` (`self.PawnReference`)
      (:`Is Valid`
        (if (`PlayerController.WasInputKeyJustPressed` _returnvalue "F")
          (set `self.PressedKeyOnce?` true)
          (if (and (`self.isCollisionWithPlayer?`) (`self.PressedKeyOnce?`))
            (`Widget.RemoveFromParent` (`self.HUD_KeyPressF`))
            (`Controller.Possess` _returnvalue self)))))))

(event `Key|D`
  (params (Key :type "Key Structure"))
  ;[1 1 1] Horizontal Rotation
  (:`Pressed`
    (if (`KismetSystemLibrary.K2_IsTimerActiveHandle` (`self.AimRightTimerHandle`))
      (`KismetSystemLibrary.K2_ClearAndInvalidateTimerHandle` (`self.AimRightTimerHandle`) :!label _label_3)
      (else
        (bind _returnvalue (`KismetSystemLibrary.K2_SetTimerDelegate` (delegate `AimRight`) (`self.HorizontalAimTime`) true))
        (set `self.AimRightTimerHandle` _returnvalue))))
  (:`Released`
    (goto _label_3)))

(event `Key|S`
  (params (Key :type "Key Structure"))
  ;[1 1 1] Vertical rotation (aiming)
  (:`Pressed`
    (if (`KismetSystemLibrary.K2_IsTimerActiveHandle` (`self.AimDownTimerHandle`))
      (`KismetSystemLibrary.K2_ClearAndInvalidateTimerHandle` (`self.AimDownTimerHandle`) :!label _label_4)
      (else
        (bind _returnvalue (`KismetSystemLibrary.K2_SetTimerDelegate` (delegate `AimDown`) (`self.VerticalAimTime`) true))
        (set `self.AimDownTimerHandle` _returnvalue))))
  (:`Released`
    (goto _label_4)))

(event `AimRight`
  ;[1 1 1] Horizontal Rotation
  (set `self.Yaw` (`KismetMathLibrary.FClamp` (+ (`self.Yaw`) (`self.DeltaAim`)) -30.0 30.0)))

(event `AimDown`
  ;[1 1 1] Vertical rotation (aiming)
  (set `self.Pitch` (`KismetMathLibrary.FClamp` (- (`self.Pitch`) (`self.DeltaAim`)) -60.0 60.0)))

(event `Key|F`
  (params (Key :type "Key Structure"))
  (bind _pawnreference (`self.PawnReference`))
  ;[1 1 1] F key press (unpossess)
  (:`Pressed`
    (`/Engine/EditorBlueprintResources/StandardMacros.IsValid` _pawnreference
      (:`Is Valid`
        (`Controller.Possess` (`self.GetController`) _pawnreference)
        (set `self.CanBePossessed` false)
        (`KismetSystemLibrary.Delay` 0.01)
        (set `self.CanBePossessed` true)
        (set `self.PressedKeyOnce?` false)))))

(event `Key|LeftMouseButton`
  (params (Key :type "Key Structure"))
  (bind _returnvalue (`SceneComponent.K2_GetComponentLocation` (`self.Arrow`)))
  ;[1 1 1] Shoot
  (:`Pressed`
    (if (`self.CanShoot`)
      (set `self.CanShoot` false)
      (set `self.IsShooting` true)
      (`GameplayStatics.PlaySoundAtLocation` (`self.ShootSound`) _returnvalue (struct) 1.0 1.0 0.0 null null null null)
      (`NiagaraFunctionLibrary.SpawnSystemAtLocation` (`self.ShootVFX`) _returnvalue (struct) (1.0 1.0 1.0) true true "AutoRelease"))))

(event `Key|Two`
  (params (Key :type "Key Structure"))
  ;[1 1 1] Camera toggles
  (:`Pressed`
    (`ActorComponent.Activate` (`self.Camera`) false)))

(event `Shoot`
  ;[1 1 1] Shoot
  (`SceneComponent.SetHiddenInGame` (`self.ArrowMesh`) true false)
  (`|SpawnActorFromClass` (`self.ArrowClass`) (`SceneComponent.K2_GetComponentToWorld` (`self.Arrow`)) "Undefined" "SelectDefaultAtRuntime" null self)
  (`KismetSystemLibrary.Delay` (`self.AfterShotDelay`))
  (set `self.IsShooting` false))

(event `self.Box.OnComponentBeginOverlap`
  (params (OverlappedComponent :type "PrimitiveComponent Object Reference") (OtherActor :type "Actor Object Reference") (OtherComp :type "PrimitiveComponent Object Reference") (OtherBodyIndex :type Integer) (bFromSweep :type Boolean) (SweepResult :type "HitResult Structure (by ref)"))
  ;[1 1 1] Overlaps
  (set `self.isCollisionWithPlayer?` true)
  (bind _returnvalue (`|CreateWidget` "/Game/InkGuard/UI/2D/WBP_KeyPress1.WBP_KeyPress1_C" (`GameplayStatics.GetPlayerController` 0)))
  (bind _output_get (set `self.HUD_KeyPressF` _returnvalue))
  (`UserWidget.AddToViewport` _output_get 0)
  (bind _aspawn (cast `Pawn` OtherActor))
  (if (`self.IsPlayerControlled` _aspawn)
    (set `self.PawnReference` _aspawn)
    (set `self.CanBePossessed` true)))

(event `EndShoot`
  ;[1 1 1] Shoot
  (set `self.CanShoot` true)
  (`SceneComponent.SetHiddenInGame` (`self.ArrowMesh`) false false))

(event `self.Box.OnComponentEndOverlap`
  (params (OverlappedComponent :type "PrimitiveComponent Object Reference") (OtherActor :type "Actor Object Reference") (OtherComp :type "PrimitiveComponent Object Reference") (OtherBodyIndex :type Integer))
  ;[1 1 1] Overlaps
  (if (== OtherActor (`self.PawnReference`))
    (set `self.PawnReference` null)
    (set `self.CanBePossessed` false)
    (set `self.isCollisionWithPlayer?` false)
    (`Widget.RemoveFromParent` (`self.HUD_KeyPressF`))))

(fn `UserConstructionScript`)