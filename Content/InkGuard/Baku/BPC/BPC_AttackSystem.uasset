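; Sword attack component for BP_Baku that runs a four-hit montage combo and resolves sword hits.
; IA_Attack or OnNetworkProcess starts attacks when CanAttack is set; input during a swing is buffered for SwordAttackCombo to chain, otherwise the combo resets.
; A fast looping timer sphere-traces between the blade points, giving Damageable hits blood, damage and camera shake, throttled by DoOnce.
; EnemyBaku owners skip damage and shake, keeping only the blood effect.
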(event `self.ReceiveBeginPlay`
  (bind _asbp_baku (cast `/Game/InkGuard/Baku/BP_Baku` (`self.GetOwner`)))
  (set `self.Character BP` _asbp_baku)
  (set `self.Character Mesh` (`Character.Mesh` _asbp_baku)))

(event `EnhancedInput|/Game/ThirdPerson/Input/Actions/IA_Attack`
  (params (ActionValue :type "Vector2D Structure") (ElapsedSeconds :type "Float (double-precision)") (TriggeredSeconds :type "Float (double-precision)") (InputAction :type "InputAction Object Reference" :default "/Game/ThirdPerson/Input/Actions/IA_Attack.IA_Attack"))
  ;[0.151 0.151 0.151] Combo System
  ;;[0.151 0.151 0.151] Attack Input
  (:`Triggered`
    (`self.Product Attack Input`)))

(event `Attack1`
  ;[0.151 0.151 0.151] Combo System
  ;;[0.151 0.151 0.151] Attack1
  (`/Engine/EditorBlueprintResources/StandardMacros.DoOnce` false :!label _label
    (:`Completed`
      (`KismetSystemLibrary.Delay` 0.1)
      (`|PlayMontage` (`self.Character Mesh`) "/Game/InkGuard/Baku/Animations/AnimationMontage/Baku_Combo2_Montage.Baku_Combo2_Montage" 1.0 0.0 "Combo1"
        (:`then`
          (set `self.attack Index` 1)
          (goto _label :!via `Reset`))))))

(event `Attack2`
  ;[0.151 0.151 0.151] Combo System
  ;;[0.151 0.151 0.151] Attack2
  (`/Engine/EditorBlueprintResources/StandardMacros.DoOnce` false :!label _label_2
    (:`Completed`
      (`KismetSystemLibrary.Delay` 0.1)
      (`|PlayMontage` (`self.Character Mesh`) "/Game/InkGuard/Baku/Animations/AnimationMontage/Baku_Combo2_Montage.Baku_Combo2_Montage" 1.0 0.0 "Combo2"
        (:`then`
          (set `self.attack Index` 2)
          (goto _label_2 :!via `Reset`))))))

(event `Sword Attack`
  ;[0.151 0.151 0.151] Combo System
  ;;[0.151 0.151 0.151] Sword Attack
  (if (`self.is Attacking?`)
    (set `self.save Attack?` true)
    (else
      (set `self.is Attacking?` true)
      (switch `int` (`self.attack Index`) :!label _label_3
        (:`0`
          (`self.Attack1`))
        (:`1`
          (`self.Attack2`))
        (:`2`
          (`self.Attack3`))
        (:`3`
          (`self.Attack4`))))))

(event `Sword Attack Combo`
  ;[0.151 0.151 0.151] Combo System
  ;;[0.151 0.151 0.151] Combo Continue
  (if (`self.save Attack?`)
    (set `self.save Attack?` false)
    (goto _label_3)
    (else
      (`self.Stop Combo`))))

(event `Attack3`
  ;[0.151 0.151 0.151] Combo System
  ;;[0.151 0.151 0.151] Attack3
  (`/Engine/EditorBlueprintResources/StandardMacros.DoOnce` false :!label _label_4
    (:`Completed`
      (`KismetSystemLibrary.Delay` 0.1)
      (`|PlayMontage` (`self.Character Mesh`) "/Game/InkGuard/Baku/Animations/AnimationMontage/Baku_Combo2_Montage.Baku_Combo2_Montage" 1.0 0.0 "Combo3"
        (:`then`
          (set `self.attack Index` 3)
          (goto _label_4 :!via `Reset`))))))

(event `Stop Combo`
  ;[0.151 0.151 0.151] Combo System
  ;;[0.151 0.151 0.151] Stop Combo/ Attack
  (set `self.is Attacking?` false)
  (set `self.attack Index` 0))

(event `Attack4`
  ;[0.151 0.151 0.151] Combo System
  ;;[0.151 0.151 0.151] Attack4
  (`/Engine/EditorBlueprintResources/StandardMacros.DoOnce` false :!label _label_5
    (:`Completed`
      (`KismetSystemLibrary.Delay` 0.1)
      (`|PlayMontage` (`self.Character Mesh`) "/Game/InkGuard/Baku/Animations/AnimationMontage/Baku_Combo2_Montage.Baku_Combo2_Montage" 1.0 0.0 "Combo4"
        (:`then`
          (set `self.attack Index` 4)
          (goto _label_5 :!via `Reset`))))))

(event `Start Sword Trace`
  ;[0.151 0.151 0.151] Sword Trace
  (bind _returnvalue (`KismetSystemLibrary.K2_SetTimerDelegate` (delegate `Sword Trace Loop`) 0.001 true))
  (set `self.SwordTraceLoop` _returnvalue))

(event `Sphere Trace`
  (bind _returnvalue (`SceneComponent.K2_GetComponentLocation` (`/Game/InkGuard/Baku/BP_Baku.Sphere Trace` (`self.Character BP`))))
  ;[1 1 1] Sphere Trace
  (bind (_outhit _returnvalue_2) (`KismetSystemLibrary.SphereTraceSingle` _returnvalue _returnvalue 25.0 "TraceTypeQuery1"))
  (if _returnvalue_2
    (bind (_bblockinghit _binitialoverlap _time _distance _location _impactpoint _normal _impactnormal _physmat _hitactor) (`GameplayStatics.BreakHitResult` _outhit))
    (if (`Actor.ActorHasTag` _hitactor "Damageable")
      (`GameplayStatics.ApplyDamage` _hitactor)
      (`GameplayStatics.PlayWorldCameraShake` "/Game/InkGuard/Baku/BP_SwordHitCameraShake.BP_SwordHitCameraShake_C" _location 0.0 2000.0))))

(event `Sword Trace Loop`
  ;[0.151 0.151 0.151] Sword Trace
  (bind (_outhit _returnvalue) (`KismetSystemLibrary.SphereTraceSingle` (`SceneComponent.K2_GetComponentLocation` (`/Game/InkGuard/Baku/BP_Baku.Sword Top Point` (`self.Character BP`))) (`SceneComponent.K2_GetComponentLocation` (`/Game/InkGuard/Baku/BP_Baku.Sword Bottom Point` (`self.Character BP`))) 12.0 "TraceTypeQuery4" false (`|MakeArray` (`self.GetOwner`)) "ForDuration" true (struct :`R` 1.0 :`A` 1.0) (struct :`G` 1.0 :`A` 1.0) 0.2))
  (if _returnvalue
    (bind (_bblockinghit _binitialoverlap _time _distance _location _impactpoint _normal _impactnormal _physmat _hitactor) (`GameplayStatics.BreakHitResult` _outhit))
    (`KismetSystemLibrary.PrintString` (`KismetSystemLibrary.GetObjectName` _hitactor))
    (if (`Actor.ActorHasTag` _hitactor "Damageable")
      (`/Engine/EditorBlueprintResources/StandardMacros.DoOnce` false :!label _label_6
        (:`Completed`
          ;;[1 0.02329 0] EnemyBaku면 데미지는 생략한다.
          (if (not (`/Game/InkGuard/Baku/BP_Baku.bEnemyBaku` (`self.Character BP`)))
            (`GameplayStatics.ApplyDamage` _hitactor 10.0 null (`self.Character BP`))
            (`GameplayStatics.PlayWorldCameraShake` "/Game/InkGuard/Baku/BP_SwordHitCameraShake.BP_SwordHitCameraShake_C" _location 0.0 2000.0))
          (`GameplayStatics.SpawnEmitterAtLocation` "/Game/Realistic_Starter_VFX_Pack_Vol2/Particles/Blood/P_Blood_Splat_Cone.P_Blood_Splat_Cone" _location (`KismetMathLibrary.MakeRotFromXY` _normal _normal) (0.4 0.4 0.4) true "AutoRelease")
          (`KismetSystemLibrary.Delay` 0.1)
          (goto _label_6 :!via `Reset`))))))

(event `Stop Sword Trace`
  ;[0.151 0.151 0.151] Sword Trace
  (`KismetSystemLibrary.K2_ClearAndInvalidateTimerHandle` (`self.SwordTraceLoop`)))

(fn `OnNetworkProcess`
  (`self.Product Attack Input`)
  (set `self.save Attack?` false))

(fn `Product Attack Input`
  (if (`self.can Attack?`)
    (`self.Sword Attack`)))