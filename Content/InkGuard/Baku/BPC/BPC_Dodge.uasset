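; BPC_Dodge is an actor component that gives BP_Baku a dodge roll triggered by the IA_Dodge input.
; When not already dodging, it stops any combo running in the owner's attack system, then plays a forward roll montage on the cached mesh.
; An IsDodging flag blocks repeat dodges and clears after a short delay once the montage completes or is interrupted.
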(event `self.ReceiveBeginPlay`
  (bind _asbp_baku (cast `/Game/InkGuard/Baku/BP_Baku` (`self.GetOwner`)))
  (set `self.As BP Baku` _asbp_baku)
  (set `self.Mesh` (`Character.Mesh` _asbp_baku)))

(event `EnhancedInput|/Game/ThirdPerson/Input/Actions/IA_Dodge`
  (params (ActionValue :type Boolean) (ElapsedSeconds :type "Float (double-precision)") (TriggeredSeconds :type "Float (double-precision)") (InputAction :type "InputAction Object Reference" :default "/Game/ThirdPerson/Input/Actions/IA_Dodge.IA_Dodge"))
  ;[0.151 0.151 0.151] Dodge
  (:`Triggered`
    (`self.Dodge Process`)))

(event `Dodge Process`
  (bind _bpc_attacksystem (`/Game/InkGuard/Baku/BP_Baku.BPC_AttackSystem` (`self.As BP Baku`)))
  ;[0.151 0.151 0.151] Dodge
  (if (not (`self.is Dodging?`))
    (if (`/Game/InkGuard/Baku/BPC/BPC_AttackSystem.is Attacking?` _bpc_attacksystem)
      (`/Game/InkGuard/Baku/BPC/BPC_AttackSystem.Stop Combo` _bpc_attacksystem))
    (`self.Play Dodge Animation`)))

(event `Play Dodge Animation`
  ;[0.151 0.151 0.151] Dodge
  (`|PlayMontage` (`self.Mesh`) "/Game/InkGuard/Baku/Animations/AnimationMontage/Dodge_Small_Forward_Roll_Montage.Dodge_Small_Forward_Roll_Montage"
    (:`then`
      (set `self.is Dodging?` true))
    (:`OnCompleted`
      (`KismetSystemLibrary.Delay` 0.2 :!label _label)
      (set `self.is Dodging?` false))
    (:`OnInterrupted`
      (goto _label))))