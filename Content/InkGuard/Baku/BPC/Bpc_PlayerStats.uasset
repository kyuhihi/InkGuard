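; Stats component holding health and stamina for Baku, EnemyBaku, SpearMan and Daka characters.
; On BeginPlay it waits a tick, then casts its owner to set a character-type enum and cache the reference.
; Change functions adjust values, with decreases returning whether depleted, and mostly route through ModifyCharacterPercent.
; That function switches on type to update Baku's HUD or SpearMan and Daka health bars; EnemyBaku has no UI branch.
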(event `self.ReceiveBeginPlay`
  (bind _returnvalue (`self.GetOwner`))
  (`KismetSystemLibrary.DelayUntilNextTick`)
  (bind _asbp_baku (cast `/Game/InkGuard/Baku/BP_Baku` (`self.GetOwner`))
    (:`then`
      (bind _output_get (set `self.Player Character BP` _asbp_baku))
      (cast `/Game/InkGuard/EnemyBP/EnemyBaku/BP_EnemyBaku` _output_get
        (:`then`
          (set `self.E_CharacterType` "NewEnumerator2"))
        (:`CastFailed`
          (set `self.E_CharacterType` "NewEnumerator0")))
      (`self.Modify Character Percent` false))
    (:`CastFailed`
      (bind _asbp_spear_man (cast `/Game/InkGuard/EnemyBP/SpearMan/BP_SpearMan` _returnvalue)
        (:`then`
          (set `self.SpearMan BP` _asbp_spear_man)
          (set `self.E_CharacterType` "NewEnumerator1"))
        (:`CastFailed`
          (bind _asbp_daka (cast `/Game/InkGuard/Daka/BP_Daka` _returnvalue))
          (set `self. BP Daka` _asbp_daka)
          (set `self.E_CharacterType` "NewEnumerator4")))))
  (`self.Modify Character Percent` true))

(fn `Decrease Health`
  (params (Damage :type "Float (double-precision)"))
  (returns (`IsPlayerDead?` :type Boolean))
  (if (not (<= (`self.Current Health`) 0.0))
    (set `self.Current Health` (- (`self.Current Health`) Damage))
    (`self.Modify Character Percent` true)
    (if (<= (`self.Current Health`) 0.0)
      _
      (else
        (return false))))
  (return true))

(fn `Decrease Stamina`
  (params (`Stamina Depleted` :type "Float (double-precision)"))
  (returns (`Not Stamina Left` :type Boolean))
  (if (not (<= (`self.Current Stamina`) 0.0))
    (set `self.Current Stamina` (- (`self.Current Stamina`) `Stamina Depleted`))
    (`self.Modify Character Percent` false)
    (if (<= (`self.Current Stamina`) 0.0)
      _
      (else
        (return false))))
  (return true))

(fn `Increase Health`
  (params (`Added Health` :type "Float (double-precision)"))
  (set `self.Current Health` (+ (`self.Current Health`) `Added Health`))
  (if (> (`self.Current Health`) (`self.Max Health`))
    (set `self.Current Health` (`self.Max Health`)))
  (`self.Modify Character Percent` true))

(fn `Increase Max Health`
  (params (`Health Incremention` :type "Float (double-precision)"))
  (set `self.Max Health` (+ (`self.Max Health`) `Health Incremention`))
  (`self.Modify Character Percent` true))

(fn `Increase Max Stamina`
  (params (`Added Stamina` :type "Float (double-precision)"))
  (set `self.Max Stamina` (+ (`self.Max Stamina`) `Added Stamina`))
  (`ProgressBar.SetPercent` (`/Game/InkGuard/Baku/WB_HUD.StaminaBar` (`/Game/InkGuard/Baku/BP_Baku.HUD Widget` (`self.Player Character BP`))) (/ (`self.Current Stamina`) (`self.Max Stamina`))))

(fn `Increase Stamina`
  (params (`Added Stamina` :type "Float (double-precision)"))
  (set `self.Current Stamina` (+ (`self.Current Stamina`) `Added Stamina`))
  (if (> (`self.Current Stamina`) (`self.Max Health`))
    (set `self.Current Stamina` (`self.Max Stamina`)))
  (`self.Modify Character Percent` false))

(fn `Modify Character Percent`
  (params (bHelthChange :type Boolean))
  (locals (HealthChange :type Boolean) (TargetProgressBar :type "ProgressBar Object Reference") (TargetPercent :type "Float (double-precision)") (TargetText :type "TextBlock Object Reference"))
  (bind _targettext (`local.TargetText`))
  (bind _hud_widget (`/Game/InkGuard/Baku/BP_Baku.HUD Widget` (`self.Player Character BP`)))
  (bind _healthbar_ui (`/Game/InkGuard/Daka/BP_Daka.HealthBar UI` (`self. BP Daka`)))
  (bind _healthbar_ui_2 (`/Game/InkGuard/EnemyBP/SpearMan/BP_SpearMan.HealthBar UI` (`self.SpearMan BP`)))
  (set `local.HealthChange` bHelthChange)
  (switch `/Game/InkGuard/Enums/BP_CharacterEnum` (`self.E_CharacterType`)
    (:`NewEnumerator0`
      (if (`local.HealthChange`)
        ;[1 0 0.06879] Health
        (set `local.TargetProgressBar` (`/Game/InkGuard/Baku/WB_HUD.HealthBar` _hud_widget))
        (set `local.TargetPercent` (/ (`self.Current Health`) (`self.Max Health`)))
        (set `local.TargetText` (`/Game/InkGuard/Baku/WB_HUD.HealthText` _hud_widget))
        (else
          ;[1 0.8883 0] Stemina
          (set `local.TargetProgressBar` (`/Game/InkGuard/Baku/WB_HUD.StaminaBar` _hud_widget))
          (set `local.TargetPercent` (/ (`self.Current Stamina`) (`self.Max Stamina`))))))
    (:`NewEnumerator1`
      (set `local.TargetProgressBar` (`/Game/InkGuard/Baku/WB_SpearManHealthBar.HealthBar` _healthbar_ui_2))
      (set `local.TargetText` (`/Game/InkGuard/Baku/WB_SpearManHealthBar.HealthText` _healthbar_ui_2))
      (set `local.TargetPercent` (/ (`self.Current Health`) (`self.Max Health`)) :!label _label))
    (:`NewEnumerator4`
      (set `local.TargetProgressBar` (`/Game/InkGuard/Baku/WB_SpearManHealthBar.HealthBar` _healthbar_ui))
      (set `local.TargetText` (`/Game/InkGuard/Baku/WB_SpearManHealthBar.HealthText` _healthbar_ui))
      (goto _label)))
  (`ProgressBar.SetPercent` (`local.TargetProgressBar`) (`local.TargetPercent`))
  (`/Engine/EditorBlueprintResources/StandardMacros.IsValid` _targettext
    (:`Is Valid`
      (set `TextBlock.Text` (`KismetTextLibrary.Conv_DoubleToText` (`self.Current Health`) "HalfToEven") _targettext))))

(fn `SetHP`
  (locals (`Target Percent` :type "Float (double-precision)"))
  (bind _healthbar_ui (`/Game/InkGuard/Daka/BP_Daka.HealthBar UI` (`self. BP Daka`)))
  (bind _healthbar_ui_2 (`/Game/InkGuard/EnemyBP/SpearMan/BP_SpearMan.HealthBar UI` (`self.SpearMan BP`)))
  (bind _hud_widget (`/Game/InkGuard/Baku/BP_Baku.HUD Widget` (`self.Player Character BP`)))
  (set `self.Current Health` (`self.Max Health`))
  (set `local.Target Percent` (/ (`self.Current Health`) (`self.Max Health`)))
  (switch `/Game/InkGuard/Enums/BP_CharacterEnum` (`self.E_CharacterType`)
    (:`NewEnumerator0`
      (`ProgressBar.SetPercent` (`/Game/InkGuard/Baku/WB_HUD.HealthBar` _hud_widget) (`local.Target Percent`))
      (set `TextBlock.Text` (`KismetTextLibrary.Conv_DoubleToText` (`self.Current Health`) "HalfToEven") (`/Game/InkGuard/Baku/WB_HUD.HealthText` _hud_widget)))
    (:`NewEnumerator1`
      (`ProgressBar.SetPercent` (`/Game/InkGuard/Baku/WB_SpearManHealthBar.HealthBar` _healthbar_ui_2) (`local.Target Percent`))
      (set `TextBlock.Text` (`KismetTextLibrary.Conv_DoubleToText` (`self.Current Health`) "HalfToEven") (`/Game/InkGuard/Baku/WB_SpearManHealthBar.HealthText` _healthbar_ui_2)))
    (:`NewEnumerator4`
      (`ProgressBar.SetPercent` (`/Game/InkGuard/Baku/WB_SpearManHealthBar.HealthBar` _healthbar_ui) (`local.Target Percent`))
      (set `TextBlock.Text` (`KismetTextLibrary.Conv_DoubleToText` (`self.Current Health`) "HalfToEven") (`/Game/InkGuard/Baku/WB_SpearManHealthBar.HealthText` _healthbar_ui)))))

(fn `Sync HP`
  (params (`Received HP` :type "Float (double-precision)"))
  (set `self.Current Health` `Received HP`)
  (`self.Modify Character Percent` true))