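; Skill component for the Baku character that handles the Q and E skill inputs, playing each skill's montage on the owner's mesh.
; Each skill is gated by a cooldown value that a Delay loop refills in steps after use.
; Q also checks the attack system's state, flags itself active until the montage ends, and uses a timer to spawn BP_Shadow afterimages at the mesh transform.
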(event `self.ReceiveBeginPlay`
  (bind _asbp_baku (cast `/Game/InkGuard/Baku/BP_Baku` (`self.GetOwner`)))
  (set `self.As BP Baku` _asbp_baku)
  (set `self.Mesh` (`Character.Mesh` _asbp_baku)))

(event `ESkillPlayMontage`
  (if (>= (`self.Skill ECool Down`) 1.0)
    (`|PlayMontage` (`self.Mesh`) "/Game/InkGuard/Baku/Animations/AnimationMontage/Baku_ESkill_Montage.Baku_ESkill_Montage"
      (:`then`
        (set `self.Skill ECool Down` 0.0)
        (if (< (`self.Skill ECool Down`) 1.0) :!label _label
          (set `self.Skill ECool Down` (+ (`self.Skill ECool Down`) 0.1))
          (`KismetSystemLibrary.Delay` 0.5)
          (goto _label))))))

(event `EnhancedInput|/Game/ThirdPerson/Input/Actions/IA_SkillE`
  (params (ActionValue :type Boolean) (ElapsedSeconds :type "Float (double-precision)") (TriggeredSeconds :type "Float (double-precision)") (InputAction :type "InputAction Object Reference" :default "/Game/ThirdPerson/Input/Actions/IA_SkillE.IA_SkillE"))
  (:`Triggered`
    (`self.ESkillPlayMontage`)))

(event `EnhancedInput|/Game/ThirdPerson/Input/Actions/IA_Skill`
  (params (ActionValue :type Boolean) (ElapsedSeconds :type "Float (double-precision)") (TriggeredSeconds :type "Float (double-precision)") (InputAction :type "InputAction Object Reference" :default "/Game/ThirdPerson/Input/Actions/IA_Skill.IA_Skill"))
  ;[0.151 0.151 0.151] Q Skill
  (:`Triggered`
    (if (>= (`self.Skill QCool Down`) 1.0)
      (`self.QSkillPlayMontage`)
      (set `self.Skill QCool Down` 0.0)
      (if (< (`self.Skill QCool Down`) 1.0) :!label _label_2
        (set `self.Skill QCool Down` (+ (`self.Skill QCool Down`) 0.1))
        (`KismetSystemLibrary.Delay` 0.2)
        (goto _label_2)))))

(event `QSkillPlayMontage`
  (bind _bpc_attacksystem (`/Game/InkGuard/Baku/BP_Baku.BPC_AttackSystem` (`self.As BP Baku`)))
  (if (not (and (`/Game/InkGuard/Baku/BPC/BPC_AttackSystem.is Attacking?` _bpc_attacksystem) (`/Game/InkGuard/Baku/BPC/BPC_AttackSystem.can Attack?` _bpc_attacksystem)))
    (set `self.IsQSkillCheck` true)
    (`KismetSystemLibrary.K2_SetTimerDelegate` (delegate `CustomEvent_2`) 0.2 (`self.IsAfterImageEffecting?`))
    (`|PlayMontage` (`self.Mesh`) "/Game/InkGuard/Baku/Animations/AnimationMontage/Baku_QSkill_Montage.Baku_QSkill_Montage"
      (:`OnCompleted`
        _)
      (:`OnBlendOut`
        _)
      (:`OnInterrupted`
        _))
    (set `self.IsAfterImageEffecting?` false)
    (set `self.IsQSkillCheck` false)))

(event `CustomEvent_2`
  ;[1 1 1] For AfterImage Effect
  (`|SpawnActorFromClass` "/Game/InkGuard/Baku/Niagara/BP_Shadow.BP_Shadow_C" (`SceneComponent.K2_GetComponentToWorld` (`self.Mesh`)) "Undefined" "MultiplyWithRoot" null null))