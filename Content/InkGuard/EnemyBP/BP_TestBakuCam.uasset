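; BP_TestBakuCam is a scene capture actor that mirrors the follow camera of the player's BP_Baku character into a render target.
; On BeginPlay it caches that camera and resizes the capture's render target once to match the viewport size.
; Every Tick it copies the camera's world transform onto the SceneCaptureComponent2D, so the capture renders from the player's viewpoint.
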(event `self.ReceiveBeginPlay`
  (bind (_sizex _sizey) (`PlayerController.GetViewportSize` (`GameplayStatics.GetPlayerController` 0)))
  (bind _asbp_baku (cast `/Game/InkGuard/Baku/BP_Baku` (`GameplayStatics.GetPlayerCharacter` 0)))
  (set `self.Follow Camera` (`/Game/InkGuard/Baku/BP_Baku.FollowCamera` _asbp_baku))
  (`KismetRenderingLibrary.ResizeRenderTarget2D` (`SceneCaptureComponent2D.TextureTarget` (`self.SceneCaptureComponent2D`)) _sizex _sizey))

(event `self.ReceiveTick`
  (params (DeltaSeconds :type "Float (single-precision)"))
  (`SceneComponent.K2_SetWorldTransform` (`self.SceneCaptureComponent2D`) (`SceneComponent.K2_GetComponentToWorld` (`self.Follow Camera`)) false false))

(fn `UserConstructionScript`)