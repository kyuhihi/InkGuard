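; BP_SpearMan is the spearman soldier AI that heads for a DoReRae territory point and fights the opposing team.
; Sensing and a timed sphere trace feed Blackboard keys; AttackPlayer cycles three montage combos, with spear overlaps applying damage.
; Lethal hits spawn a death-animation actor, then respawn the same pawn at its spawner or saved transform and restart AI.
; Enemy-flagged instances can mirror position, yaw, speed and montage time from received packets.
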(event `self.ReceiveBeginPlay`
  (`self.SEt Dorerae`)
  ;[1 1 1] UI
  (bind _aswb_spear_man_health_bar (cast `/Game/InkGuard/Baku/WB_SpearManHealthBar` (`WidgetComponent.GetWidget` (`self.Health Bar Widget`))))
  (set `self.HealthBar UI` _aswb_spear_man_health_bar)
  (`KismetSystemLibrary.K2_SetTimer` null "CheckCanAttack" (`self.CheckCanAttackTimer`) true)
  (bind _asink_guard_game_mode (cast `InkGuardGameMode` (`GameplayStatics.GetGameMode`)))
  (bind _returnvalue (`InkGuardGameMode.GetCurGameMode` _asink_guard_game_mode))
  (switch `EMainGameState` _returnvalue
    (:`GAME_WAITING`
      (set `self.Save Spawner Pos` (`self.GetTransform`))
      (`self.BBSetTargetDorere` "NewEnumerator0"))
    (:`GAME_MAINGAME`
      (`KismetSystemLibrary.K2_SetTimerDelegate` (delegate `Check Only MainGame Actor`) 3.0))))

(event `Check Only MainGame Actor`
  (`/Engine/EditorBlueprintResources/StandardMacros.IsValid` (`self.MySpawner`)
    (:`Is Not Valid`
      (`self.K2_DestroyActor`))))

(event `self.ReceiveTick`
  (params (DeltaSeconds :type "Float (single-precision)"))
  (`self.SetHpBarBillboard`)
  (if (not (`self.bEnemySpearMan`))
    (set `self.Speed` (`KismetMathLibrary.VSize` (`MovementComponent.Velocity` (`self.CharacterMovement`))))))

(event `self.PawnSensing.OnSeePawn`
  (params (Pawn :type "Pawn Object Reference"))
  (bind _returnvalue (`AIBlueprintHelperLibrary.GetBlackboard` (`AIBlueprintHelperLibrary.GetAIController` self)))
  (if (`KismetSystemLibrary.DoesImplementInterface` Pawn "/Script/InkGuard.SoldierInterface")
    (bind _returnvalue_2 (message `SoldierInterface.IsOurTeam` Pawn))
    (bind _returnvalue_3 (`self.IsOurTeam`))
    (if (!= _returnvalue_3 _returnvalue_2)
      (`self.SetBlackBoardValueBool` null (`self.BB_HasSeenPlayer`) true)
      (`/Engine/EditorBlueprintResources/StandardMacros.IsValid` _returnvalue
        (:`Is Valid`
          (`BlackboardComponent.SetValueAsObject` _returnvalue (`self.BB_TargetActorName`) Pawn))))))

(event `AttackPlayer`
  ;[1 1 1] AttackPawn
  (if (<= (`/Game/InkGuard/Baku/BPC/Bpc_PlayerStats.Current Health` (`self.Bpc_PlayerStats`)) 0.0)
    (`self.StopAttack Montage`)
    (else
      (bind _isplaying (`self.IsPlayingComboAttackMontage`))
      (if (not _isplaying)
        (`self.SetBlackBoardValueBool` null (`self.BB_IsPlayingComboAttackMontage`) true)
        (`self.ChooseAttackMontage`
          (:`0`
            (`self.HeavyAttackCombo`
              (:`OnBlendOut`
                _)))
          (:`1`
            (`self.AttackCombo`
              (:`OnBlendOut`
                _)))
          (:`2`
            (`self.DodgeAttackCombo`
              (:`OnBlendOut`
                _))))
        (`self.SetBlackBoardValueBool` null (`self.BB_IsPlayingComboAttackMontage`))))))

(event `self.ReceiveAnyDamage`
  (params (Damage :type "Float (single-precision)") (DamageType :type "DamageType Object Reference") (InstigatedBy :type "Controller Object Reference") (DamageCauser :type "Actor Object Reference"))
  ;[1 1 1] Damaged
  (if (`KismetSystemLibrary.DoesImplementInterface` DamageCauser "/Script/InkGuard.SoldierInterface")
    (bind _returnvalue (message `SoldierInterface.IsOurTeam` DamageCauser))
    (bind _returnvalue_2 (`self.IsOurTeam`))
    (if (!= _returnvalue_2 _returnvalue)
      (`self.SetDamagedLoutine` Damage DamageCauser DamageCauser))))

(event `self.SpearCollision.OnComponentBeginOverlap`
  (params (OverlappedComponent :type "PrimitiveComponent Object Reference") (OtherActor :type "Actor Object Reference") (OtherComp :type "PrimitiveComponent Object Reference") (OtherBodyIndex :type Integer) (bFromSweep :type Boolean) (SweepResult :type "HitResult Structure (by ref)"))
  ;[1 1 1] OnCollisionPawn
  (bind (_outhit _returnvalue) (`KismetSystemLibrary.LineTraceSingle` :`Start` (`SceneComponent.K2_GetComponentLocation` (`self.SpearCollision`)) :`End` (`self.K2_GetActorLocation` OtherActor) :`TraceChannel` "TraceTypeQuery4" :`DrawTime` 15.0))
  (if _returnvalue
    (bind (_bblockinghit _binitialoverlap _time _distance _location _impactpoint _normal) (`GameplayStatics.BreakHitResult` _outhit))
    (`self.Make Ink Effect` _location (1.5 1.5 1.5) (`KismetMathLibrary.MakeRotFromXY` _normal _normal))
    (`GameplayStatics.ApplyDamage` OtherActor 10.0 null self)))

(event `SoldierInterface.SetAboutSpawner`
  (params (pOwnerSpawner :type "Actor Object Reference"))
  ;[0 1 0.1864] Call By Spawner
  (bind _asbp_soldier_spawner (cast `/Game/InkGuard/MapBP/Object/SpawnPoint/BP_SoldierSpawner` pOwnerSpawner))
  (bind _output_get (set `self.MySpawner` _asbp_soldier_spawner))
  (`self.BBSetTargetDorere` (`/Game/InkGuard/MapBP/Object/SpawnPoint/BP_SoldierSpawner.eTargetTerritoryType` _output_get)))

(event `SoldierInterface.SetAboutColor`
  (params (NewColor :type Integer))
  ;[0 1 0.1864] Call By Spawner
  (switch `int` NewColor
    (:`0`
      (set `self.TeamColor` "NewEnumerator3"))
    (:`1`
      (set `self.TeamColor` "NewEnumerator0"))
    (:`2`
      (set `self.TeamColor` "NewEnumerator1"))))

(event `SoldierInterface.Respawn`
  (bind _myspawner (`self.MySpawner`))
  ;[1 0.01165 0] Respawn
  (`/Engine/EditorBlueprintResources/StandardMacros.IsValid` (`self.MySpawner`)
    (:`Is Valid`
      (bind _returnvalue (`/Game/InkGuard/MapBP/Object/SpawnPoint/BP_SoldierSpawner.GetRespawn Point` _myspawner))
      (`self.K2_SetActorTransform` _returnvalue false true)
      (`self.BBSetTargetDorere` (`/Game/InkGuard/MapBP/Object/SpawnPoint/BP_SoldierSpawner.eTargetTerritoryType` _myspawner)))
    (:`Is Not Valid`
      (`self.K2_SetActorTransform` (`self.Save Spawner Pos`) false true)))
  (`/Game/InkGuard/Baku/BPC/Bpc_PlayerStats.SetHP` (`self.Bpc_PlayerStats`))
  (`self.RestartAI`))

(event `self.SensingSphere.OnComponentBeginOverlap`
  (params (OverlappedComponent :type "PrimitiveComponent Object Reference") (OtherActor :type "Actor Object Reference") (OtherComp :type "PrimitiveComponent Object Reference") (OtherBodyIndex :type Integer) (bFromSweep :type Boolean) (SweepResult :type "HitResult Structure (by ref)"))
  (bind _returnvalue (`AIBlueprintHelperLibrary.GetBlackboard` (`AIBlueprintHelperLibrary.GetAIController` self)))
  (bind _returnvalue_2 (message `SoldierInterface.IsOurTeam` OtherActor))
  (bind _returnvalue_3 (`self.IsOurTeam`))
  (if (!= _returnvalue_2 _returnvalue_3)
    (`self.SetBlackBoardValueBool` null (`self.BB_HasSeenPlayer`) true)
    (`/Engine/EditorBlueprintResources/StandardMacros.IsValid` _returnvalue
      (:`Is Valid`
        (`BlackboardComponent.SetValueAsObject` _returnvalue (`self.BB_TargetActorName`) OtherActor)))))

(event `SoldierInterface.SetValueOfPacket`
  (params (tRecvPacket :type "PACKET_SOLDIER_TRANSFORM_BLUEPRINT Structure"))
  ;[1 1 1] Packet
  (if (`self.bEnemySpearMan`)
    (`self.K2_SetActorLocation` tRecvPacket_vSoldier_Position)
    (`self.K2_SetActorRotation` (`KismetMathLibrary.MakeRotator` 0.0 0.0 tRecvPacket_fSoldier_Yaw))
    (set `self.Speed` tRecvPacket_fSoldier_Speed)
    (if (> tRecvPacket_fSoldier_MontagePlayTime 0.0)
      (`|PlayMontage` (`self.Mesh`) "/Game/InkGuard/EnemyBP/SpearMan/Animation/AM_SpearMan_Combo_Heavy.AM_SpearMan_Combo_Heavy" 1.0 tRecvPacket_fSoldier_MontagePlayTime)
      (else
        (`/Engine/EditorBlueprintResources/StandardMacros.IsValid` (`AnimInstance.GetCurrentActiveMontage` (`SkeletalMeshComponent.GetAnimInstance` (`self.Mesh`)))
          (:`Is Valid`
            (`self.StopAnimMontage` (`self.GetCurrentMontage`))))))))

(event `SoldierInterface.SpawnerTick`
  (params (fTimeDelta :type "Float (single-precision)"))
  (bind (_returnvalue_roll _returnvalue_pitch _returnvalue_yaw) (`KismetMathLibrary.BreakRotator` (`self.GetControlRotation`)))
  ;[1 1 1] If Without Update
  (`self.AddMovementInput` (`KismetMathLibrary.GetForwardVector` (`KismetMathLibrary.MakeRotator` 0.0 0.0 _returnvalue_yaw))))

(fn `AboutKeyPressingF`
  (returns (ReturnValue :type Boolean))
  (return false))

(fn `BBSetTargetDorere`
  (params (Selection :type "/Game/InkGuard/Enums/BP_TerritoryType Enum" :default "NewEnumerator0"))
  (bind _bb_maingametargetdoreraeposition (`self.BB_MainGameTargetDoreraePosition`))
  (bind _returnvalue (`AIBlueprintHelperLibrary.GetBlackboard` (`AIBlueprintHelperLibrary.GetAIController` self)))
  (`/Engine/EditorBlueprintResources/StandardMacros.IsValid` (`AIBlueprintHelperLibrary.GetBlackboard` (`AIBlueprintHelperLibrary.GetAIController` null))
    (:`Is Valid`
      (if (<= (`KismetArrayLibrary.Array_Length` (`self.Doreraes Actors`)) 0)
        (bind _outactors (`GameplayStatics.GetAllActorsOfClass` "/Game/InkGuard/MapBP/Object/DoReRae/BP_DoReRae.BP_DoReRae_C"))
        (set `self.Doreraes Actors` _outactors))
      (for _array_element (`self.Doreraes Actors`)
        (switch `/Game/InkGuard/Enums/BP_TerritoryType` Selection
          (:`NewEnumerator0`
            (bind _doreraetype (`/Game/InkGuard/MapBP/Object/DoReRae/BP_DoReRae.DoreraeType` _array_element))
            (switch `/Game/InkGuard/MapBP/Object/DoReRae/E_DoreraeType` _doreraetype
              (:`NewEnumerator0`
                (bind _returnvalue_2 (`SceneComponent.K2_GetComponentLocation` (`/Game/InkGuard/MapBP/Object/DoReRae/BP_DoReRae.AI MovePoint Sphere` _array_element)))
                (`BlackboardComponent.SetValueAsVector` _returnvalue _bb_maingametargetdoreraeposition _returnvalue_2))))
          (:`NewEnumerator1`
            (switch `/Game/InkGuard/MapBP/Object/DoReRae/E_DoreraeType` _doreraetype
              (:`NewEnumerator1`
                (`BlackboardComponent.SetValueAsVector` _returnvalue _bb_maingametargetdoreraeposition _returnvalue_2))))
          (:`NewEnumerator4`
            (switch `/Game/InkGuard/MapBP/Object/DoReRae/E_DoreraeType` _doreraetype
              (:`NewEnumerator2`
                (`BlackboardComponent.SetValueAsVector` _returnvalue _bb_maingametargetdoreraeposition _returnvalue_2)))))))))

(fn `CheckCanAttack`
  (bind _returnvalue (`self.K2_GetActorLocation`))
  (bind _bb_canattack (`self.BB_CanAttack`))
  ;[1 0 0.0124] CheckDead
  (if (<= (`/Game/InkGuard/Baku/BPC/Bpc_PlayerStats.Current Health` (`self.Bpc_PlayerStats`)) 0.0)
    (`self.SetBlackBoardValueBool` null (`self.BB_CanAttack`))
    (else
      (bind (_outhit _returnvalue_2) (`KismetSystemLibrary.SphereTraceSingleForObjects` _returnvalue (+ _returnvalue (* (`KismetMathLibrary.GetForwardVector` (`self.K2_GetActorRotation`)) 50.0)) 300.0 (`|MakeArray` "ObjectTypeQuery3" :!type "EObjectTypeQuery Enum")))
      (if _returnvalue_2
        (bind `_as폰` (cast `Pawn` (`.HitActor` (`GameplayStatics.BreakHitResult` _outhit)))
          (:`then`
            (if (`KismetSystemLibrary.DoesImplementInterface` `_as폰` "/Script/InkGuard.SoldierInterface")
              (bind _returnvalue_3 (message `SoldierInterface.IsDead` `_as폰`))
              (if (not _returnvalue_3)
                (bind _returnvalue_4 (`self.IsOurTeam`))
                (bind _returnvalue_5 (message `SoldierInterface.IsOurTeam` `_as폰`))
                (if (!= _returnvalue_4 _returnvalue_5)
                  (set `self.TargetPawn` `_as폰`)
                  (`self.SetBlackBoardValueBool` null _bb_canattack true)))))
          (:`CastFailed`
            (`self.SetBlackBoardValueBool` null _bb_canattack :!label _label)))
        (else
          (goto _label))))))

(fn `GetColor`
  (returns (ReturnValue :type Integer))
  (return 0))

(fn `GetHP`
  (returns (ReturnValue :type "Float (single-precision)"))
  (return (`/Game/InkGuard/Baku/BPC/Bpc_PlayerStats.Current Health` (`self.Bpc_PlayerStats`))))

(fn `GetPlayerInputData`
  (returns (ReturnValue :type "PlayerInputStruct Structure"))
  (return))

(fn `IsDead`
  (returns (ReturnValue :type Boolean))
  (return (<= (`/Game/InkGuard/Baku/BPC/Bpc_PlayerStats.Current Health` (`self.Bpc_PlayerStats`)) 0.0)))

(fn `IsOurTeam`
  (returns (ReturnValue :type Boolean))
  (return (not (`self.bEnemySpearMan`))))

(fn `IsPlayingComboAttackMontage`
  (returns (IsPlaying :type Boolean))
  (bind _returnvalue (`AIBlueprintHelperLibrary.GetBlackboard` (`AIBlueprintHelperLibrary.GetAIController` self)))
  (`/Engine/EditorBlueprintResources/StandardMacros.IsValid` _returnvalue
    (:`Is Valid`
      (return (`BlackboardComponent.GetValueAsBool` _returnvalue (`self.BB_IsPlayingComboAttackMontage`))))
    (:`Is Not Valid`
      (return (`AnimInstance.IsAnyMontagePlaying` (`SkeletalMeshComponent.GetAnimInstance` (`self.Mesh`)))))))

(fn `LookAtTarget`
  (bind _targetpawn (`self.TargetPawn`))
  (bind (_returnvalue_roll _returnvalue_pitch _returnvalue_yaw) (`KismetMathLibrary.BreakRotator` (`KismetMathLibrary.FindLookAtRotation` (`self.K2_GetActorLocation`) (`self.K2_GetActorLocation` _targetpawn))))
  (`/Engine/EditorBlueprintResources/StandardMacros.IsValid` _targetpawn
    (:`Is Valid`
      (`self.K2_SetActorRotation` (`KismetMathLibrary.MakeRotator` 0.0 0.0 _returnvalue_yaw)))
    (:`Is Not Valid`
      (set `self.TargetPawn` null)
      (`self.SetBlackBoardValueBool` null (`self.BB_CanAttack`)))))

(fn `Make Ink Effect`
  (params (Location :type "Vector Structure") (Scale :type "Vector Structure") (Rotation :type "Rotator Structure"))
  (`GameplayStatics.SpawnEmitterAtLocation` "/Game/Realistic_Starter_VFX_Pack_Vol2/Particles/Blood/P_Blood_Splat_Cone.P_Blood_Splat_Cone" Location Rotation Scale true "AutoRelease"))

(fn `RestartAI`
  (bind _returnvalue (`AIBlueprintHelperLibrary.GetAIController` self))
  (bind _returnvalue_2 (`AIBlueprintHelperLibrary.GetBlackboard` _returnvalue))
  (`/Engine/EditorBlueprintResources/StandardMacros.IsValid` _returnvalue_2
    (:`Is Valid`
      (`BrainComponent.RestartLogic` (`AIController.BrainComponent` _returnvalue))
      (`BlackboardComponent.ClearValue` _returnvalue_2 (`self.BB_HasSeenPlayer`))
      (`BlackboardComponent.ClearValue` _returnvalue_2 (`self.BB_CanAttack`))
      (`BlackboardComponent.ClearValue` _returnvalue_2 (`self.BB_TargetLastPosition`))
      (`BlackboardComponent.ClearValue` _returnvalue_2 (`self.BB_TargetActorName`)))))

(fn `SEt Dorerae`
  (bind _returnvalue (`AIBlueprintHelperLibrary.GetBlackboard` null))
  (`/Engine/EditorBlueprintResources/StandardMacros.IsValid` (`AIBlueprintHelperLibrary.GetBlackboard` null)
    (:`Is Valid`
      (bind _outactors (`GameplayStatics.GetAllActorsOfClass` "/Game/InkGuard/MapBP/Object/DoReRae/BP_DoReRae.BP_DoReRae_C"))
      (for _array_element _outactors
        (switch `/Game/InkGuard/MapBP/Object/DoReRae/E_DoreraeType` (`/Game/InkGuard/MapBP/Object/DoReRae/BP_DoReRae.DoreraeType` _array_element)
          (:`NewEnumerator0`
            (`BlackboardComponent.SetValueAsObject` _returnvalue "DoReRaeA" _array_element))
          (:`NewEnumerator1`
            (`BlackboardComponent.SetValueAsObject` _returnvalue "DoReRaeB" _array_element))
          (:`NewEnumerator2`
            (`BlackboardComponent.SetValueAsObject` _returnvalue "DoReRaeC" _array_element)))))))

(fn `SetAttackPlayingMontageAndStopMontage`
  (bind _isplaying (`self.IsPlayingComboAttackMontage`))
  (if _isplaying
    (`self.StopAttack Montage`)))

(fn `SetBlackBoardValueBool`
  (params (Object :type "Object Object Reference") (BB_Name :type Name) (SetValue :type Boolean))
  (bind _returnvalue (`AIBlueprintHelperLibrary.GetBlackboard` (`AIBlueprintHelperLibrary.GetAIController` self)))
  (`/Engine/EditorBlueprintResources/StandardMacros.IsValid` Object
    (:`Is Valid`
      (cast `/Game/ThirdPerson/Blueprints/BP_ThirdPersonCharacter` Object)
      (`/Engine/EditorBlueprintResources/StandardMacros.IsValid` _returnvalue
        (:`Is Valid`
          (`BlackboardComponent.SetValueAsBool` _returnvalue BB_Name SetValue))))
    (:`Is Not Valid`
      (`/Engine/EditorBlueprintResources/StandardMacros.IsValid` _returnvalue
        (:`Is Valid`
          (`BlackboardComponent.SetValueAsBool` _returnvalue BB_Name SetValue))))))

(fn `SetBlackBoardValueVector`
  (params (KeyName :type "Name (by ref)") (Value :type "Vector Structure"))
  (bind _returnvalue (`AIBlueprintHelperLibrary.GetBlackboard` (`AIBlueprintHelperLibrary.GetAIController` self)))
  (`/Engine/EditorBlueprintResources/StandardMacros.IsValid` _returnvalue
    (:`Is Valid`
      (`BlackboardComponent.SetValueAsVector` _returnvalue KeyName Value))))

(fn `SetDamagedLoutine`
  (params (InputPin :type "Float (single-precision)") (self2 :type "Actor Object Reference") (self3 :type "Actor Object Reference"))
  (bind _braincomponent (`AIController.BrainComponent` (`AIBlueprintHelperLibrary.GetAIController` self)))
  (`self.SetAttackPlayingMontageAndStopMontage`)
  (`self.LaunchCharacter` (* (`KismetMathLibrary.GetForwardVector` (`self.K2_GetActorRotation` self3)) 700.0))
  ;[1 0 0.04792] Set Dead
  (bind _isplayerdead_ (`/Game/InkGuard/Baku/BPC/Bpc_PlayerStats.Decrease Health` (`self.Bpc_PlayerStats`) InputPin))
  (if _isplayerdead_
    (`self.K2_SetActorRotation` (`KismetMathLibrary.FindLookAtRotation` (`self.K2_GetActorLocation`) (`self.K2_GetActorLocation` self2)))
    (`PrimitiveComponent.SetSimulatePhysics` (`self.Mesh`) true)
    (`ActorComponent.SetActive` (`self.NS_SpearTrail`) false false)
    (`/Engine/EditorBlueprintResources/StandardMacros.IsValid` _braincomponent
      (:`Is Valid`
        (`BrainComponent.StopLogic` _braincomponent ""))
      (:`Is Not Valid`
        _))
    (`|SpawnActorFromClass` "/Game/InkGuard/EnemyBP/SpearMan/BP_AISpearMandeadAnimation.BP_AISpearMandeadAnimation_C" (`self.GetTransform`) "AdjustIfPossibleButAlwaysSpawn" "MultiplyWithRoot" null null)
    (`self.Respawn`)))

(fn `StopAttack Montage`
  (`self.StopAnimMontage` (`self.GetCurrentMontage`))
  (`self.SetBlackBoardValueBool` null (`self.BB_IsPlayingComboAttackMontage`))
  (`self.SetBlackBoardValueBool` null (`self.BB_CanAttack`)))

(fn `UserConstructionScript`)