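; BP_EnemyBaku is the networked opponent Baku, mirroring a remote player through its PlayerNetwork component.
; While waiting, Tick polls for game start and opens the main map; in the main game it exchanges transform and input packets with the local player's data.
; Received attack packets drive BPCAttackSystem and align the active montage to the sender's playback time.
; Sprint Niagara toggling is present but unconnected.
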(event `self.ReceiveBeginPlay`
  (`ActorComponent.Deactivate` (`self.Niagara`))
  (set `self.bEnemyBaku` true)
  (bind _asbp_baku (cast `/Game/InkGuard/Baku/BP_Baku` (`GameplayStatics.GetPlayerPawn` 0)))
  (bind _output_get (set `self.BP Baku` _asbp_baku))
  (`PlayerNetwork.SetPlayerStruct` (`self.PlayerNetwork`) (make `PlayerStruct` _output_get))
  (bind _asink_guard_game_mode (cast `InkGuardGameMode` (`GameplayStatics.GetGameMode`)))
  (set `self.As Ink Guard Game Mode` _asink_guard_game_mode))

(event `self.ReceiveTick`
  (params (DeltaSeconds :type "Float (single-precision)"))
  (bind _playernetwork (`self.PlayerNetwork`))
  (`parent.ReceiveTick` DeltaSeconds)
  (bind _returnvalue (`InkGuardGameMode.GetCurGameMode` (`self.As Ink Guard Game Mode`)))
  (switch `EGameState` _returnvalue
    (:`GAME_WAITING`
      (bind _returnvalue_2 (`PlayerNetwork.CheckGameStart` _playernetwork))
      (if _returnvalue_2
        (`GameplayStatics.OpenLevel` "Level_MainMap")))
    (:`GAME_MAINGAME`
      (`self.Sync Transform` DeltaSeconds)
      (`self.Sync Input` DeltaSeconds)
      (`PlayerNetwork.TidyNetworkTickRoutine` _playernetwork))))

(fn `Conduct Input Packet`
  (params (RecvPacket :type "PlayerInputStruct Structure"))
  (bind (_pressingf _attack _vault _dodge _sprint _montageplaytime) (break `PlayerInputStruct` RecvPacket))
  (bind _returnvalue (`SkeletalMeshComponent.GetAnimInstance` (`self.Mesh`)))
  ;[1 1 1] attack
  (if _attack
    (`/Game/InkGuard/Baku/BPC/BPC_AttackSystem.OnNetworkProcess` (`self.BPC_AttackSystem`))
    (set `self.isPressingF` _pressingf)
    ;[1 0.01768 0] AnimationSync
    (`AnimInstance.Montage_SetPosition` _returnvalue (`AnimInstance.GetCurrentActiveMontage` _returnvalue) _montageplaytime)))

(fn `GetPlayerInputData`
  (returns (ReturnValue :type "PlayerInputStruct Structure"))
  (return))

(fn `Sync Input`
  (params (DeltaTime :type "Float (single-precision)"))
  (bind _playernetwork (`self.PlayerNetwork`))
  (bind _returnvalue (`PlayerInterface.GetPlayerInputData` (`self.BP Baku`)))
  (`PlayerNetwork.SendPlayerInputData` _playernetwork 0.0 _returnvalue)
  ;[1 1 1] Others
  (bind _toutinputs (`PlayerNetwork.RecvPlayerInputData` _playernetwork DeltaTime))
  (`self.Conduct Input Packet` _toutinputs))

(fn `Sync Transform`
  (params (DeltaTime :type "Float (single-precision)"))
  (bind _playernetwork (`self.PlayerNetwork`))
  (`PlayerNetwork.SendPlayerTransform` _playernetwork DeltaTime)
  (`PlayerNetwork.RecvPlayerTransform` _playernetwork DeltaTime)
  ;[1 0.09669 0] Sync Location & Rotation
  (bind _returnvalue (`PlayerNetwork.GetPlayerStruct` (`self.PlayerNetwork`)))
  (set `self.VelocityZ` (`.fVelocityZ` (break `PlayerStruct` _returnvalue)))
  (set `self.Speed` (`.fSpeed` (break `PlayerStruct` _returnvalue))))

(fn `UserConstructionScript`
  (`parent.UserConstructionScript`))